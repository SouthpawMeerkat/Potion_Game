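; Sigil plate actor that can be painted on at runtime and keeps a score for good and bad hits.
; BeginPlay creates a render target, feeds it into the cylinder's dynamic material, and gathers the correct-line and bad collision boxes into arrays.
; DrawBrush stamps a brush material onto the render target at a normalized location.
; Points adds for good hits and deducts a penalty for bad ones.
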(event `self.ReceiveBeginPlay`
  (bind _correctline (`self.CorrectLine`))
  (bind _badboxcollision (`self.BadBoxCollision`))
  (`|ExecutionSequence`
    (:`then_0`
      (bind _returnvalue (`KismetRenderingLibrary.CreateRenderTarget2D` 512 512))
      (bind _output_get (set `self.RenderTarget` _returnvalue))
      (`KismetRenderingLibrary.ClearRenderTarget2D` _output_get (struct :`R` 0.15625 :`G` 0.031488 :`B` 0.001756 :`A` 1.0)))
    (:`then_1`
      (bind _returnvalue_2 (`KismetMaterialLibrary.CreateDynamicMaterialInstance` "/Game/Stokes/M_SigilPlate.M_SigilPlate"))
      (`MaterialInstanceDynamic.SetTextureParameterValue` _returnvalue_2 "SigilBasePlate" (`self.RenderTarget`))
      (`PrimitiveComponent.SetMaterial` (`self.Cylinder`) 0 _returnvalue_2))
    (:`then_2`
      (bind _returnvalue_3 (`KismetMaterialLibrary.CreateDynamicMaterialInstance` "/Game/Stokes/M_Drawn.M_Drawn"))
      (set `self.DrawMat` _returnvalue_3))
    (:`then_3`
      (bind _output_get_2 (set `self.GoodCollisionBoxes` (`SceneComponent.GetChildrenComponents` _correctline false)))
      (`KismetArrayLibrary.Array_AddUnique` _output_get_2 _correctline))
    (:`then_4`
      (bind _output_get_3 (set `self.BadCollisionBoxes` (`SceneComponent.GetChildrenComponents` _badboxcollision false)))
      (`KismetArrayLibrary.Array_AddUnique` _output_get_3 _badboxcollision))))

(fn `DrawBrush`
  (params (BrushTexture :type "Texture2D Object Reference") (BrushSize :type "Float (double-precision)") (DrawLocation :type "Vector2D Structure"))
  (bind _brushsize (`local.BrushSize`))
  (`|ExecutionSequence`
    (:`then_0`
      (`MaterialInstanceDynamic.SetTextureParameterValue` (`self.DrawMat`) "BrushTexture" BrushTexture))
    (:`then_1`
      (bind (_canvas _size _context) (`KismetRenderingLibrary.BeginDrawCanvasToRenderTarget` (`self.RenderTarget`)))
      (`Canvas.K2_DrawMaterial` _canvas (`self.DrawMat`) (- (* _size (`local.DrawLocation`)) (/ _brushsize 2.0)) (`KismetMathLibrary.MakeVector2D` _brushsize _brushsize) (0.0 0.0) (1.0 1.0) 0.0 (0.5 0.5))
      (`KismetRenderingLibrary.EndDrawCanvasToRenderTarget` _context))))

(fn `Points`
  (params (bIsGoodHit :type Boolean))
  (if bIsGoodHit
    (`/Engine/EditorBlueprintResources/StandardMacros.IncrementInt` (`self.TotalPoints`)
      (:`  `
        (`/Engine/EditorBlueprintResources/StandardMacros.IncrementInt` (`self.GoodHits`))))
    (else
      (set `self.TotalPoints` (- (`self.TotalPoints`) (`self.BadHitPointLoss`))))))

(fn `UserConstructionScript`)