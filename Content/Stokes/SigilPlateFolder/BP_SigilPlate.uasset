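; BP_SigilPlate is a timed sigil-drawing plate that scores the player's drawing.
; BeginPlay sets up a render-target-backed material, key points, a timer and a temporary three-second self-destruct.
; DrawBrush paints brush textures onto the target, while Points counts hits and returns the player once no key points remain.
; Completion or timeout triggers Reset, which rates time and hits as an outcome number, then clears the canvas.
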(event `self.ReceiveBeginPlay`
  (bind _sphere (`self.Sphere`))
  (`|ExecutionSequence`
    (:`then_0`
      (bind _returnvalue (`KismetRenderingLibrary.CreateRenderTarget2D` 512 512))
      (bind _output_get (set `self.RenderTarget` _returnvalue))
      (`KismetRenderingLibrary.ClearRenderTarget2D` _output_get (struct :`R` 0.15625 :`G` 0.031488 :`B` 0.001756 :`A` 1.0)))
    (:`then_1`
      (bind _returnvalue_2 (`KismetMaterialLibrary.CreateDynamicMaterialInstance` "/Game/Stokes/M_SigilPlate.M_SigilPlate"))
      (`MaterialInstanceDynamic.SetTextureParameterValue` _returnvalue_2 "SigilBasePlate" (`self.RenderTarget`))
      (`PrimitiveComponent.SetMaterial` (`self.Cylinder`) 0 _returnvalue_2))
    (:`then_2`
      (bind _returnvalue_3 (`KismetMaterialLibrary.CreateDynamicMaterialInstance` "/Game/Stokes/M_Drawn.M_Drawn"))
      (set `self.DrawMat` _returnvalue_3))
    (:`then_3`
      (bind _output_get_2 (set `self.KeyPoints` (`SceneComponent.GetChildrenComponents` _sphere false)))
      (`KismetArrayLibrary.Array_AddUnique` _output_get_2 _sphere))
    (:`then_4`
      (bind _returnvalue_4 (`KismetSystemLibrary.K2_SetTimerDelegate` (delegate `Drawing Started`) (`self.TimerLength`)))
      (set `self.TimerHandle` _returnvalue_4))
    (:`then_5`
      ;[1 1 1] Stops endless sigils being created (will be deleted once sigil drawing can be completed)
      (`KismetSystemLibrary.Delay` 3.0)
      (`self.K2_DestroyActor`))))

(event `Drawing Started`
  (set `self.TimeElapsed` (`KismetSystemLibrary.K2_GetTimerElapsedTimeHandle` (`self.TimerHandle`)))
  (`self.reset`))

(fn `DrawBrush`
  (params (BrushTexture :type "Texture2D Object Reference") (BrushSize :type "Float (double-precision)") (DrawLocation :type "Vector2D Structure"))
  (bind _brushsize (`local.BrushSize`))
  (if (`self.bDrawingInProgress`)
    (`|ExecutionSequence`
      (:`then_0`
        (`MaterialInstanceDynamic.SetTextureParameterValue` (`self.DrawMat`) "BrushTexture" BrushTexture))
      (:`then_1`
        (bind (_canvas _size _context) (`KismetRenderingLibrary.BeginDrawCanvasToRenderTarget` (`self.RenderTarget`)))
        (`Canvas.K2_DrawMaterial` _canvas (`self.DrawMat`) (- (* _size (`local.DrawLocation`)) (/ _brushsize 2.0)) (`KismetMathLibrary.MakeVector2D` _brushsize _brushsize) (0.0 0.0) (1.0 1.0) 0.0 (0.5 0.5))
        (`KismetRenderingLibrary.EndDrawCanvasToRenderTarget` _context)))))

(fn `outcomeCalculator`
  (if (>= (`self.TimeElapsed`) (`self.HighestGoodTime`))
    (if (< (`self.HitKeyPointCount`) (`self.MaxPoints`))
      ;[1 1 1] To long, Missing Keypoints
      (set `self.OutputNumberKey` 1)
      (else
        ;[1 1 1] To Long, With All keypoints
        (set `self.OutputNumberKey` 2)))
    (elif (>= (`self.TimeElapsed`) (`self.LowestGoodTime`))
      ;[1 1 1] Just right
      (set `self.OutputNumberKey` 3)
      (else
        ;[1 1 1] To fast
        (set `self.OutputNumberKey` 4)))))

(fn `Points`
  (if true
    (`/Engine/EditorBlueprintResources/StandardMacros.IncrementInt` (`self.HitKeyPointCount`)
      (:`  `
        (if (<= (`KismetArrayLibrary.Array_Length` (`self.KeyPoints`)) 0)
          (bind _asbp_sigil_player_character (cast `/Game/Stokes/BP_SigilPlayerCharacter` (`GameplayStatics.GetPlayerPawn` 0)))
          (`/Game/Stokes/BP_SigilPlayerCharacter.Return` _asbp_sigil_player_character)
          (set `self.TimeElapsed` (`KismetSystemLibrary.K2_GetTimerElapsedTimeHandle` (`self.TimerHandle`)))
          (`self.reset`)
          (`KismetSystemLibrary.K2_ClearAndInvalidateTimerHandle` (`self.TimerHandle`)))))))

(fn `reset`
  (`self.outcomeCalculator`)
  (`KismetSystemLibrary.PrintText` (`KismetTextLibrary.Conv_IntToText` (`self.OutputNumberKey`)))
  (`KismetRenderingLibrary.ClearRenderTarget2D` (`self.RenderTarget`) (struct :`R` 0.15625 :`G` 0.031488 :`B` 0.001756 :`A` 1.0))
  (bind _returnvalue (`GameplayStatics.GetActorOfClass` "BP_SigilPlate_C"))
  (`self.SetActorHiddenInGame` false)
  (if (not (== _returnvalue self))
    (`self.K2_DestroyActor`)))

(fn `UserConstructionScript`)