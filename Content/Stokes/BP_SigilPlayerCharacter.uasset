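; Player character for a sigil-drawing and ingredient-crushing game, driven by mouse clicks through Enhanced Input.
; Clicking while idle traces under the cursor and maps the hit actor's class to a current action, which the back input clears.
; Sigil mode paints a brush on the plate at the hit UV and scores good or bad collision boxes, disabling each hit box.
; Crushing mode opens the game mode's mortar-and-pestle widget.
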(event `self.ReceiveBeginPlay`
  (`EnhancedInputSubsystemInterface.AddMappingContext` (pcsubsystem `EnhancedInputLocalPlayerSubsystem` (`GameplayStatics.GetPlayerController` 0)) "/Game/Stokes/IM_Click.IM_Click" 0 (struct))
  (bind _asbp_sigil_gmb (cast `/Game/Stokes/BP_SigilGMB` (`GameplayStatics.GetGameMode`)))
  (set `self.As BP Sigil GMB` _asbp_sigil_gmb))

(event `EnhancedInput|/Game/Stokes/IA_Click`
  (params (ActionValue :type Boolean) (ElapsedSeconds :type "Float (double-precision)") (TriggeredSeconds :type "Float (double-precision)") (InputAction :type "InputAction Object Reference" :default "/Game/Stokes/IA_Click.IA_Click"))
  (bind (_worldlocation _worlddirection) (`PlayerController.DeprojectMousePositionToWorld` (`GameplayStatics.GetPlayerController` 0)))
  (bind _mortarandpestle (`/Game/Stokes/BP_SigilGMB.MortarAndPestle` (`self.As BP Sigil GMB`)))
  (:`Triggered`
    (switch `string` (`self.CurrentAction`)
      (:`Sigil`
        (`self.DrawingSigil`))
      (:`Crushing`
        (if (not (`Widget.IsInViewport` _mortarandpestle))
          (`UserWidget.AddToViewport` _mortarandpestle 0)))))
  (:`Started`
    (if (`KismetStringLibrary.EqualEqual_StrStr` (`self.CurrentAction`))
      (bind _outhit (`KismetSystemLibrary.LineTraceSingle` (`SceneComponent.K2_GetComponentLocation` (`self.PlayerViewPort`)) (+ (* _worlddirection (10000.0 10000.0 10000.0)) _worldlocation) "TraceTypeQuery1"))
      (bind _output_get (set `self.CurrentAction` (`BlueprintMapLibrary.Map_Find` (`self.ClassToAction`) (`KismetSystemLibrary.GetClassDisplayName` (`GameplayStatics.GetObjectClass` (`.HitActor` (`GameplayStatics.BreakHitResult` _outhit)))))))
      (`KismetSystemLibrary.PrintString` (`KismetStringLibrary.Concat_StrStr` "You Are Now " _output_get))
      (`KismetSystemLibrary.Delay` 0.2))))

(event `EnhancedInput|/Game/Stokes/IA_Move`
  (params (ActionValue :type "Vector2D Structure") (ElapsedSeconds :type "Float (double-precision)") (TriggeredSeconds :type "Float (double-precision)") (InputAction :type "InputAction Object Reference" :default "/Game/Stokes/IA_Move.IA_Move"))
  (bind (_returnvalue_roll _returnvalue_pitch _returnvalue_yaw) (`KismetMathLibrary.BreakRotator` (`self.GetControlRotation`)))
  (bind _returnvalue_roll_2 (`KismetMathLibrary.BreakRotator` (`self.GetControlRotation`)))
  ;[1 1 1] To Be Deleted
  (:`Triggered`
    (`self.AddMovementInput` (`KismetMathLibrary.GetRightVector` (`KismetMathLibrary.MakeRotator` _returnvalue_roll 0.0 _returnvalue_yaw)) ActionValue_X)
    (`self.AddMovementInput` (`KismetMathLibrary.GetForwardVector` (`KismetMathLibrary.MakeRotator` _returnvalue_roll_2)) ActionValue_Y)))

(event `EnhancedInput|/Game/Stokes/IA_Back`
  (params (ActionValue :type Boolean) (ElapsedSeconds :type "Float (double-precision)") (TriggeredSeconds :type "Float (double-precision)") (InputAction :type "InputAction Object Reference" :default "/Game/Stokes/IA_Back.IA_Back"))
  ;[1 1 1] To Be Deleted
  (:`Triggered`
    (`self.Return`)))

(event `EnhancedInput|/Game/Stokes/IA_Inventory`
  (params (ActionValue :type Boolean) (ElapsedSeconds :type "Float (double-precision)") (TriggeredSeconds :type "Float (double-precision)") (InputAction :type "InputAction Object Reference" :default "/Game/Stokes/IA_Inventory.IA_Inventory"))
  ;[1 1 1] To Be Deleted
  (:`Started`
    (`/Game/Stokes/WB_Inventory.Visable` (`/Game/Stokes/BP_SigilGMB.InventoryRef` (`self.As BP Sigil GMB`)))))

(fn `DrawingSigil`
  (bind _returnvalue (`SceneComponent.K2_GetComponentLocation` (`self.PlayerViewPort`)))
  (bind (_worldlocation _worlddirection) (`PlayerController.DeprojectMousePositionToWorld` (`GameplayStatics.GetPlayerController` 0)))
  (bind _returnvalue_2 (+ (* _worlddirection (10000.0 10000.0 10000.0)) _worldlocation))
  (`|ExecutionSequence`
    (:`then_0`
      (bind _outhit (`KismetSystemLibrary.LineTraceSingle` _returnvalue _returnvalue_2 "TraceTypeQuery1"))
      (bind _asbp_sigil_plate (cast `/Game/Stokes/BP_SigilPlate` (`.HitActor` (`GameplayStatics.BreakHitResult` _outhit))))
      (`/Game/Stokes/BP_SigilPlate.DrawBrush` _asbp_sigil_plate (`self.Brush Texture`) (`self.Brush Size`) (`GameplayStatics.FindCollisionUV` _outhit)))
    (:`then_1`
      (bind _outhit_2 (`KismetSystemLibrary.LineTraceSingle` _returnvalue _returnvalue_2 "TraceTypeQuery3"))
      (bind (_bblockinghit _binitialoverlap _time _distance _location _impactpoint _normal _impactnormal _physmat _hitactor _hitcomponent) (`GameplayStatics.BreakHitResult` _outhit_2))
      (bind _asbp_sigil_plate_2 (cast `/Game/Stokes/BP_SigilPlate` _hitactor))
      (if (`KismetMathLibrary.Conv_IntToBool` (`KismetArrayLibrary.Array_Find` (`/Game/Stokes/BP_SigilPlate.GoodCollisionBoxes` _asbp_sigil_plate_2) _hitcomponent))
        (bind _output_get (set `self.bGoodHit` true))
        (`/Game/Stokes/BP_SigilPlate.Points` _asbp_sigil_plate_2 _output_get)
        (`PrimitiveComponent.SetCollisionEnabled` _hitcomponent "NoCollision" :!label _label)
        (elif (`KismetMathLibrary.Conv_IntToBool` (`KismetArrayLibrary.Array_Find` (`/Game/Stokes/BP_SigilPlate.BadCollisionBoxes` _asbp_sigil_plate_2) _hitcomponent))
          (bind _output_get_2 (set `self.bGoodHit` false))
          (`/Game/Stokes/BP_SigilPlate.Points` _asbp_sigil_plate_2 _output_get_2)
          (goto _label))))))

(fn `GrindHeldIngrediant`
  (params (Percent :type "Float (double-precision)"))
  (bind _asbp_ingrediants (cast `/Game/Stokes/BP_Ingrediants` (`self.IngrediantHeld`)))
  (set `/Game/Stokes/BP_Ingrediants.GroundPercent` Percent _asbp_ingrediants))

(fn `Return`
  (set `self.CurrentAction` ""))

(fn `UserConstructionScript`)