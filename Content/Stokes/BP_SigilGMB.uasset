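; BP_SigilGMB manages sigil swapping and holds the UI widgets for the sigil game.
; On BeginPlay it creates and stores the mortar and pestle, inventory and sigil selector widgets without displaying them.
; ChangeSigil hides the BP_SigilPlate actor it finds, without destroying it, and spawns the passed class at that plate's transform.
; OpenSlashClose adds the inventory to the viewport or removes it, based on the Closing flag.
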(event `self.ReceiveBeginPlay`
  (bind _returnvalue (`|CreateWidget` "/Game/Blueprints/UI/WB_MorterAndPestel.WB_MorterAndPestel_C"))
  (set `self.MortarAndPestle` _returnvalue)
  (bind _returnvalue_2 (`|CreateWidget` "/Game/Stokes/WB_Inventory.WB_Inventory_C"))
  (set `self.InventoryUIRef` _returnvalue_2)
  (bind _returnvalue_3 (`|CreateWidget` "/Game/Blueprints/UI/UI_Sigil_Selector.UI_Sigil_Selector_C"))
  (set `self.SigilUIRef` _returnvalue_3))

(fn `Change Sigil`
  (params (SigilChangeRef :type "Actor Class Reference"))
  (bind _returnvalue (`GameplayStatics.GetActorOfClass` "/Game/Blueprints/SigilPlateFolder/BP_SigilPlate.BP_SigilPlate_C"))
  (`self.SetActorHiddenInGame` _returnvalue true)
  (`|SpawnActorFromClass` SigilChangeRef (`SceneComponent.K2_GetComponentToWorld` (`/Game/Blueprints/SigilPlateFolder/BP_SigilPlate.DefaultSceneRoot` _returnvalue)) "Undefined" "MultiplyWithRoot" null null))

(fn `OpenSlashClose`
  (params (Closing :type Boolean))
  (if Closing
    (`Widget.RemoveFromParent` (`self.InventoryUIRef`))
    (else
      (`UserWidget.AddToViewport` (`self.InventoryUIRef`) 0))))

(fn `UserConstructionScript`)