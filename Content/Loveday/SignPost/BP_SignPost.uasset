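; Signpost actor that displays a message while the player character stands within its box trigger.
; Entering the box shows the widget component and copies the SignpostMessage variable into the DisplayText of its BPW_SignPost widget, printing an error if the cast fails.
; Leaving the box hides the widget, and overlaps from other actors are ignored.
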(event `self.Box.OnComponentBeginOverlap`
  (params (OverlappedComponent :type "PrimitiveComponent Object Reference") (OtherActor :type "Actor Object Reference") (OtherComp :type "PrimitiveComponent Object Reference") (OtherBodyIndex :type Integer) (bFromSweep :type Boolean) (SweepResult :type "HitResult Structure (by ref)"))
  (bind _widget (`self.Widget`))
  (if (== OtherActor (`GameplayStatics.GetPlayerCharacter` 0))
    (`SceneComponent.SetVisibility` _widget true false)
    (bind _asbpw_sign_post (cast `/Game/Loveday/SignPost/BPW_SignPost` (`WidgetComponent.GetUserWidgetObject` _widget))
      (:`then`
        (set `/Game/Loveday/SignPost/BPW_SignPost.DisplayText` (`self.SignpostMessage`) _asbpw_sign_post))
      (:`CastFailed`
        (`KismetSystemLibrary.PrintString` "Signpost text issue")))))

(event `self.Box.OnComponentEndOverlap`
  (params (OverlappedComponent :type "PrimitiveComponent Object Reference") (OtherActor :type "Actor Object Reference") (OtherComp :type "PrimitiveComponent Object Reference") (OtherBodyIndex :type Integer))
  (if (== OtherActor (`GameplayStatics.GetPlayerCharacter` 0))
    (`SceneComponent.SetVisibility` (`self.Widget`) false false)))

(fn `UserConstructionScript`)