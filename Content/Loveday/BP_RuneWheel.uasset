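; BP_RuneWheel is an interactive rune wheel with outer and inner dials that rotate when clicked.
; RotateDial turns the clicked dial in 45-degree steps, only while the inspect component's rune movement reference reports a held rune.
; It converts the dial's rotation into an integer index, which it prints and returns, though the click events ignore it.
; UpdateSelectedRune is an uncalled stub that loops over rune data table row names.
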(event `self.ReceiveBeginPlay`)

(event `self.DialOuter.OnClicked`
  (params (TouchedComponent :type "PrimitiveComponent Object Reference") (ButtonPressed :type "Key Structure"))
  (`self.RotateDial` (`self.DialOuter`)))

(event `self.DialInner.OnClicked`
  (params (TouchedComponent :type "PrimitiveComponent Object Reference") (ButtonPressed :type "Key Structure"))
  (`self.RotateDial` (`self.DialInner`)))

(fn `RotateDial`
  (params (NewParam :type "StaticMeshComponent Object Reference"))
  (returns (PositionIndex :type Integer))
  (bind _returnvalue (/ (+ (`KismetMathLibrary.FTrunc` (`KismetMathLibrary.NormalizeAxis` (`KismetMathLibrary.GetYawPitchFromVector` (`.Y` (`KismetMathLibrary.BreakRotIntoAxes` (`SceneComponent.RelativeRotation` NewParam)))))) 135) 45))
  ;[1 1 1] Only if holding
  (if (`/Game/Loveday/BP_RuneMovement.isHoldingRune` (`/Game/Loveday/BPComponent_InspectRune.BP_RuneMovementRef` (`self.BPComponent_Inspect`)))
    (`SceneComponent.K2_AddLocalRotation` NewParam (struct :`Yaw` 45.0) false false)
    (`KismetSystemLibrary.PrintString` (`KismetStringLibrary.Conv_IntToString` _returnvalue) true true (struct :`G` 0.66 :`B` 1.0 :`A` 1.0) 3.0)
    (return _returnvalue)))

(fn `UpdateSelectedRune`
  (bind _outrownames (`DataTableFunctionLibrary.GetDataTableRowNames` (`self.RuneDataTable `)))
  (for _ _outrownames
    _))

(fn `UserConstructionScript`)