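; BP_ComponentInspect is a component that makes its owning actor respond to mouse clicks, apparently as groundwork for inspecting objects.
; On BeginPlay it binds to the owner's OnClicked event, caches the owner's static mesh component and prints that component's name.
; Each click toggles an IsClicked flag and prints it if the mesh reference is valid, with no inspection behavior beyond this debug output.
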(event `self.ReceiveBeginPlay`
  (bind _returnvalue (`self.GetOwner`))
  (bind _returnvalue_2 (`Actor.GetComponentByClass` _returnvalue "/Script/Engine.StaticMeshComponent"))
  (add `Actor.OnClicked` _returnvalue (delegate `onMouseClick`))
  (`/Engine/EditorBlueprintResources/StandardMacros.IsValid` _returnvalue_2
    (:`Is Valid`
      (set `self.StaticMeshRef` _returnvalue_2)
      (`KismetSystemLibrary.PrintString` (`KismetSystemLibrary.GetDisplayName` _returnvalue_2)))))

(event `onMouseClick`
  (params (TouchedActor :type "Actor Object Reference") (ButtonPressed :type "Key Structure" :default "None"))
  (bind _isclicked (`self.isClicked`))
  (set `self.isClicked` (not _isclicked))
  (`/Engine/EditorBlueprintResources/StandardMacros.IsValid` (`self.StaticMeshRef`)
    (:`Is Valid`
      (`KismetSystemLibrary.PrintString` (`KismetStringLibrary.Conv_BoolToString` _isclicked)))))