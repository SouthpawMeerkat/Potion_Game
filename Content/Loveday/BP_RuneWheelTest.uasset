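; Test Blueprint for a rune wheel with clickable outer and inner dials that turn in opposite directions.
; Clicks call RotateDial, which steps that ring 45 degrees only while the inspect component reports it is held.
; It then derives an integer position from the ring's rotation, printing and returning it, though callers ignore the result.
; UpdateSelectedRune is an uncalled stub that loops over rune data table row names without acting.
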(event `self.ReceiveBeginPlay`)

(event `self.ReceiveTick`
  (params (DeltaSeconds :type "Float (single-precision)")))

(event `self.DialOuter.OnClicked`
  (params (TouchedComponent :type "PrimitiveComponent Object Reference") (ButtonPressed :type "Key Structure"))
  (`self.RotateDial` (`self.DialOuter`) 1))

(event `self.DialInner.OnClicked`
  (params (TouchedComponent :type "PrimitiveComponent Object Reference") (ButtonPressed :type "Key Structure"))
  (`self.RotateDial` (`self.DialInner`) -1))

(fn `RotateDial`
  (params (Ring :type "StaticMeshComponent Object Reference") (Direction :type Integer))
  (returns (PositionIndex :type Integer))
  (bind _returnvalue (/ (+ (`KismetMathLibrary.FTrunc` (`KismetMathLibrary.NormalizeAxis` (`KismetMathLibrary.GetYawPitchFromVector` (`.Y` (`KismetMathLibrary.BreakRotIntoAxes` (`SceneComponent.RelativeRotation` Ring)))))) 135) 45))
  ;[1 1 1] Only if holding
  (if (`/Game/Blueprints/BPComponent_Inspect.isHolding` (`self.BPComponent_Inspect`))
    (`SceneComponent.K2_AddLocalRotation` Ring (`KismetMathLibrary.MakeRotator` 0.0 0.0 (`KismetMathLibrary.Conv_IntToDouble` (* Direction 45))) false false)
    (`KismetSystemLibrary.PrintString` (`KismetStringLibrary.Conv_IntToString` _returnvalue) true true (struct :`G` 0.66 :`B` 1.0 :`A` 1.0) 3.0)
    (return _returnvalue)))

(fn `UpdateSelectedRune`
  (bind _outrownames (`DataTableFunctionLibrary.GetDataTableRowNames` (`self.RuneDataTable `)))
  (for _ _outrownames
    _))

(fn `UserConstructionScript`)