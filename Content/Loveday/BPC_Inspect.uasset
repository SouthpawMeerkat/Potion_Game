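; Actor component that makes its owning actor inspectable when clicked.
; On BeginPlay it binds to the owner's OnClicked event, which triggers InspectActor.
; InspectActor finds the BP_InspectionManager with GetActorOfClass and passes it the owner, its root component, and the component's custom vector and rotator.
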(event `self.ReceiveBeginPlay`
  ;[1 1 1] mouse click event calls inspect actor
  (add `Actor.OnClicked` (`self.GetOwner`) (delegate `onMouseClick`)))

(event `InspectActor`
  (params (TouchedActor :type "Actor Object Reference"))
  (bind _returnvalue (`self.GetOwner`))
  ;[1 1 1] Pass parent details to inspections manager
  (bind _returnvalue_2 (`GameplayStatics.GetActorOfClass` "/Game/Loveday/BP_InspectionManager.BP_InspectionManager_C"))
  (`/Game/Loveday/BP_InspectionManager.InspectNewObject ` _returnvalue_2 _returnvalue (`self.CustomVector`) (`self.CustomRotator`) (`Actor.RootComponent` _returnvalue)))

(event `onMouseClick`
  (params (TouchedActor :type "Actor Object Reference") (ButtonPressed :type "Key Structure" :default "None"))
  ;[1 1 1] mouse click event calls inspect actor
  (`self.InspectActor` TouchedActor))