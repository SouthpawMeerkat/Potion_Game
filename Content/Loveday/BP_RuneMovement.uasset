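; BP_RuneMovement is a player-input Blueprint for interacting with held runes, with most of its logic disconnected.
; BeginPlay adds the IM_Main Enhanced Input mapping context to the first player controller.
; The IA_CloseD action clears IsHoldingRune and sends CloseWindowMessage to HoldingRef.
; IA_InteractD is empty, and the mouse look, camera line trace interaction and debug prints are unwired, so they never run.
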(event `EnhancedInput|/Game/Blueprints/Actions/IA_CloseD`
  (params (ActionValue :type Boolean) (ElapsedSeconds :type "Float (double-precision)") (TriggeredSeconds :type "Float (double-precision)") (InputAction :type "InputAction Object Reference" :default "/Game/Blueprints/Actions/IA_CloseD.IA_CloseD"))
  ;[1 1 1] Close button
  (:`Started`
    ;;[1 1 1] do i even need this bool?
    (if (`self.isHoldingRune`)
      (set `self.isHoldingRune` false)
      (message `/Game/Loveday/BPI_Input.CloseWindow` (`self.HoldingRef`)))))

(event `self.ReceiveBeginPlay`
  ;[1 1 1] Connect Controller
  (`EnhancedInputSubsystemInterface.AddMappingContext` (pcsubsystem `EnhancedInputLocalPlayerSubsystem` (`GameplayStatics.GetPlayerController` 0)) "/Game/Blueprints/Actions/IM_Main.IM_Main" 0 (struct)))

(event `EnhancedInput|/Game/Blueprints/Actions/IA_InteractD`
  (params (ActionValue :type Boolean) (ElapsedSeconds :type "Float (double-precision)") (TriggeredSeconds :type "Float (double-precision)") (InputAction :type "InputAction Object Reference" :default "/Game/Blueprints/Actions/IA_InteractD.IA_InteractD")))

(fn `UserConstructionScript`)