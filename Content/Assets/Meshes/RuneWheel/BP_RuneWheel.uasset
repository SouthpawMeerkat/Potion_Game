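; BP_RuneWheel is an inspectable puzzle prop with two clickable dials that select a rune and light an orb in its colour.
; While the object is held, clicks turn the dials in opposite directions by one of ten slices, deriving indices from ring rotation.
; The index pair is matched against data table rows, setting the orb's dynamic material emissive.
; A valid combination fires the RuneSelected dispatcher.
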(event `self.ReceiveBeginPlay`
  (bind _returnvalue (`PrimitiveComponent.CreateDynamicMaterialInstance` (`self.Sphere`) 0 "/Game/Loveday/Material/M_RuneOrb.M_RuneOrb" "None"))
  (bind _output_get (set `self.DMI_RuneOrb` _returnvalue))
  (`PrimitiveComponent.SetMaterial` (`self.Sphere`) 0 _output_get))

(event `self.Wheel1.OnClicked`
  (params (TouchedComponent :type "PrimitiveComponent Object Reference") (ButtonPressed :type "Key Structure"))
  (bind _positionindex (`self.RotateDial` (`self.Wheel1`) 1))
  (set `self.Wheel1Index` _positionindex)
  (bind (_runecolour _runeid) (`self.UpdateSelectedRune` :!label _label))
  (if (`self.RuneFound`)
    (`self.RuneSelected` _runeid)))

(event `self.Wheel2.OnClicked`
  (params (TouchedComponent :type "PrimitiveComponent Object Reference") (ButtonPressed :type "Key Structure"))
  (bind _positionindex (`self.RotateDial` (`self.Wheel2`) -1))
  (set `self.Wheel2Index` _positionindex)
  (goto _label))

(fn `RotateDial`
  (params (Ring :type "StaticMeshComponent Object Reference") (Direction :type Integer))
  (returns (PositionIndex :type Integer))
  ;[1 1 1] Only if holding
  (if (`/Game/Blueprints/BPComponent_Inspect.isHolding` (`self.BPComponent_Inspect`))
    ;[1 1 1] 10 slices = 36  degrees
    (`SceneComponent.K2_AddLocalRotation` Ring (`KismetMathLibrary.MakeRotator` (`KismetMathLibrary.Conv_IntToDouble` (* Direction 36))) false false)
    (return (/ (+ (`KismetMathLibrary.Round` (`KismetMathLibrary.NormalizeAxis` (`KismetMathLibrary.GetYawPitchFromVector` (`.Y` (`KismetMathLibrary.BreakRotIntoAxes` (`SceneComponent.RelativeRotation` Ring)))))) 162) 36))))

(fn `UpdateSelectedRune`
  (returns (RuneColour :type "/Game/Loveday/Data/RuneColourEnum Enum") (RuneID :type "/Game/Loveday/Data/RuneStruct Structure"))
  (bind _rune_data_table_ref (`self.Rune Data Table Ref`))
  (bind _dmi_runeorb (`self.DMI_RuneOrb`))
  (set `self.Temp Rune ID` (make `/Game/Loveday/Data/RuneStruct` "Not A Rune" "NewEnumerator4" -1))
  (set `self.RuneFound` false)
  (bind _outrownames (`DataTableFunctionLibrary.GetDataTableRowNames` _rune_data_table_ref))
  (for _array_element _outrownames
    (bind _returnvalue (`|GetDataTableRow` _rune_data_table_ref _array_element)
      (:`then`
        (bind (_runename _runecolour _runeid _wheel1position _wheel2position) (break `/Game/Loveday/Data/RuneStruct` _returnvalue))
        (if (and (== _wheel1position (`self.Wheel1Index`)) (== _wheel2position (`self.Wheel2Index`)))
          (set `self.Temp Rune ID` _returnvalue)
          (break)))))
  (bind _output_get (set `self.Selected Rune ID` (`self.Temp Rune ID`)))
  (`MaterialInstanceDynamic.SetVectorParameterValue` _dmi_runeorb "RuneOrbEmissive" (select `/Game/Loveday/Data/RuneColourEnum` (`.RuneColour_8_B8E1195845BE5C298D646A9FEFD24543` (break `/Game/Loveday/Data/RuneStruct` _output_get)) :`NewEnumerator0` (struct :`R` 1.0 :`B` 0.076702 :`A` 1.0) :`NewEnumerator1` (struct :`G` 1.0 :`B` 0.001301 :`A` 1.0) :`NewEnumerator2` (struct :`G` 0.036187 :`B` 1.0 :`A` 1.0) :`NewEnumerator3` (struct :`R` 1.0 :`G` 0.858508 :`A` 1.0) :!type "LinearColor Structure"))
  (`MaterialInstanceDynamic.SetScalarParameterValue` _dmi_runeorb "RuneOrbScalar" 1000.0)
  (set `self.RuneFound` (`.isValidCombination_19_984E02D84D26D4F38A0598B4575F0A38` (break `/Game/Loveday/Data/RuneStruct` _output_get)))
  (return "NewEnumerator4" _returnvalue))

(fn `UserConstructionScript`)