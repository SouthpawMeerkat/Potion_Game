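; BP_IngredientCombiner is an early-stage Blueprint for pairing two ingredient enum values into a text label.
; On BeginPlay it prints IngredientCombo on screen in red as a debug message.
; The logic that joins IngredientsA, "and" and IngredientsB into IngredientCombo is disconnected, so the print shows the variable's unmodified value.
; The construction script is empty.
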(event `self.ReceiveBeginPlay`
  (`KismetSystemLibrary.PrintString` (`KismetTextLibrary.Conv_TextToString` (`self.IngredientCombo`)) true true (struct :`R` 1.0 :`G` 0.015727 :`A` 1.0)))

(fn `UserConstructionScript`)