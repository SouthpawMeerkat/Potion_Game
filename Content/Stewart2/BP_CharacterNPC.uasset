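; BP_CharacterNPC is an NPC Blueprint meant to follow the spline of a referenced SplineToFollow object.
; Each Tick, while that reference is valid, it updates a distance value and sets the actor's world location and rotation from the spline at that distance.
; The update multiplies the sum of stored distance and MovementSpeed by DeltaSeconds, so the distance does not accumulate as steady travel.
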(event `self.ReceiveTick`
  (params (DeltaSeconds :type "Float (single-precision)"))
  (bind _splinetofollow (`self.SplineToFollow`))
  (`/Engine/EditorBlueprintResources/StandardMacros.IsValid` (`self.SplineToFollow`)
    (:`Is Valid`
      (bind _output_get (set `self.DIstanceAlongSpline` (* (+ (`self.DIstanceAlongSpline`) (`self.MovementSpeed`)) DeltaSeconds)))
      (`self.K2_SetActorLocationAndRotation` (`SplineComponent.GetLocationAtDistanceAlongSpline` (`/Game/Stewart2/BP_SplinePath.Spline` _splinetofollow) _output_get "World") (`SplineComponent.GetRotationAtDistanceAlongSpline` (`/Game/Stewart2/BP_SplinePath.Spline` _splinetofollow) _output_get "World")))))

(fn `UserConstructionScript`)