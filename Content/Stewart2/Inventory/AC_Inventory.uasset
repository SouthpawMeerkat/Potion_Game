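; AC_Inventory is a player character component that stores stackable items in a slot-keyed map and toggles the UMG_Inventory screen through Enhanced Input.
; The open widget receives the map and reports add, drop and remove events back to the component.
; PickupItem scans slots in order, topping up matching stacks until it reaches an empty slot, with debug prints throughout.
; Dropped items respawn as A_Item where a downward box trace ahead of the owner hits.
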(event `self.ReceiveBeginPlay`
  ;[1 1 1] Attach to player character to enable inventory
  (`EnhancedInputSubsystemInterface.AddMappingContext` (pcsubsystem `EnhancedInputLocalPlayerSubsystem` (`GameplayStatics.GetPlayerController` 0)) "/Game/Stewart2/Inventory/IMC_Inventory.IMC_Inventory" 0 (struct))
  (`KismetSystemLibrary.PrintString` (`KismetStringLibrary.Conv_IntToString` (`self.MaxSize`)))
  ;[1 1 1] Added this.. things happen. for somereason the default 30 does not come across and instead sets to 0
  (set `self.MaxSize` 30)
  (`KismetSystemLibrary.PrintString` "------START-------"))

(event `EnhancedInput|/Game/Stewart2/Inventory/IA_Inventory`
  (params (ActionValue :type Boolean) (ElapsedSeconds :type "Float (double-precision)") (TriggeredSeconds :type "Float (double-precision)") (InputAction :type "InputAction Object Reference" :default "/Game/Stewart2/Inventory/IA_Inventory.IA_Inventory"))
  (bind _returnvalue (`GameplayStatics.GetPlayerController` 0))
  (bind _returnvalue_2 (`GameplayStatics.GetPlayerController` 0))
  (bind _as_umg_inventory (`self.As UMG_Inventory`))
  (:`Started`
    (`self.As UMG_Inventory`
      (:`then`
        ;[1 1 1] Return to play
        (set `PlayerController.bShowMouseCursor` false _returnvalue)
        (`WidgetBlueprintLibrary.SetInputMode_GameOnly` _returnvalue true)
        (`Widget.RemoveFromParent` (`self.As UMG_Inventory`))
        (set `self.As UMG_Inventory` null))
      (:`else`
        (bind _returnvalue_3 (`|CreateWidget` "/Game/Stewart2/Inventory/Widgets/UMG_Inventory.UMG_Inventory_C" null (`self.Inventory`) (`self.MaxSize`) (`self.AllowDuplicates`)))
        (bind _output_get (set `self.As UMG_Inventory` _returnvalue_3))
        (`UserWidget.AddToViewport` _output_get 0)
        ;[1 1 1] Add / Drop / Remove items
        (add `/Game/Stewart2/Inventory/Widgets/UMG_Inventory.ItemAdded` _as_umg_inventory (`|CreateDelegate` :!event `ItemAdded`))
        (add `/Game/Stewart2/Inventory/Widgets/UMG_Inventory.ItemDropped` _as_umg_inventory (`|CreateDelegate` :!event `ItemDropped`))
        (add `/Game/Stewart2/Inventory/Widgets/UMG_Inventory.ItemRemoved` _as_umg_inventory (`|CreateDelegate` :!event `ItemRemoved`))
        ;[1 1 1] Sets control to inventory menu
        (set `PlayerController.bShowMouseCursor` true _returnvalue_2)
        (`WidgetBlueprintLibrary.SetInputMode_UIOnlyEx` _returnvalue_2 null)))))

(fn `Is Key Full`
  (params (Key :type Integer))
  (returns (ReturnValue :type Boolean) (Remaining :type Integer))
  (bind (_value _returnvalue) (`BlueprintMapLibrary.Map_Find` (`self.Inventory`) Key))
  (bind (_quantity _dataassets) (break `/Game/Stewart2/Inventory/Items/ST_Inventory` _value))
  (bind _maxstack (`/Game/Stewart2/Inventory/Items/DA_Items.MaxStack` _dataassets))
  (bind _returnvalue_2 (- _maxstack _quantity))
  (if _returnvalue
    (return (and (== _returnvalue_2 0) (!= _maxstack 0)) _returnvalue_2)
    (else
      (return false -1))))

(fn `ItemAdded`
  (params (`Slot Key` :type Integer) (`Slot Value` :type "/Game/Stewart2/Inventory/Items/ST_Inventory Structure"))
  (`BlueprintMapLibrary.Map_Add` (`self.Inventory`) `Slot Key` `Slot Value`))

(fn `ItemDropped`
  (params (`Item Dropped` :type "/Game/Stewart2/Inventory/Items/ST_Inventory Structure"))
  (bind _returnvalue (`self.GetOwner`))
  (bind _returnvalue_2 (+ (* (`Actor.GetActorForwardVector` _returnvalue) 300.0) (`Actor.K2_GetActorLocation` _returnvalue)))
  ;[1 1 1] Calculate location to drop item
  (bind (_outhit _returnvalue_3) (`KismetSystemLibrary.BoxTraceSingle` _returnvalue_2 (- _returnvalue_2 (0.0 0.0 500.0)) (15.0 15.0 15.0) (struct) "TraceTypeQuery1" false (`|MakeArray` (`self.GetOwner`))))
  ;[1 1 1] create new object at location
  (if _returnvalue_3
    (`|SpawnActorFromClass` "/Game/Stewart2/Inventory/Items/A_Item.A_Item_C" (`KismetMathLibrary.MakeTransform` (`.ImpactPoint` (`GameplayStatics.BreakHitResult` _outhit))) "Undefined" "MultiplyWithRoot" null (`local.Item Dropped`) null)))

(fn `ItemRemoved`
  (params (Key :type Integer))
  (`BlueprintMapLibrary.Map_Remove` (`self.Inventory`) Key))

(fn `PickupItem`
  (params (Item :type "/Game/Stewart2/Inventory/Items/A_Item Object Reference"))
  (returns (`Return Value` :type Boolean))
  (locals (`L-QuantityIn` :type Integer) (`L-DataAssetIn` :type "/Game/Stewart2/Inventory/Items/DA_Items Object Reference") (`L-Index` :type Integer :default 0) (`L-FoundSameItem` :type Boolean) (`L-Remaining` :type Integer :default 0) (`L-EmptyKey` :type Integer :default -1))
  (bind _l_quantityin (`local.L-QuantityIn`))
  (bind (_quantity _dataassets) (break `/Game/Stewart2/Inventory/Items/ST_Inventory` (`/Game/Stewart2/Inventory/Items/A_Item.Structure` Item)))
  (bind (_returnvalue _remaining) (`self.Is Key Full` (`local.L-Index`)))
  (bind _value (`BlueprintMapLibrary.Map_Find` (`self.Inventory`) (`local.L-Index`)))
  (bind _returnvalue_2 (- (`local.L-QuantityIn`) (`local.L-Remaining`)))
  ;[1 1 1] Create local vars from item structure
  (set `local.L-QuantityIn` _quantity)
  (set `local.L-DataAssetIn` _dataassets)
  ;[1 1 1] Loop whilst items can be picked up and there is room in map
  (while (and (> (`local.L-QuantityIn`) 0) (< (`local.L-Index`) (`self.MaxSize`)))
    ;[0 1 0.15] pick up details at start of while loop
    (`KismetSystemLibrary.PrintString` "----------" true true (struct :`G` 1.0 :`B` 0.14996 :`A` 1.0) 5.0)
    (`KismetSystemLibrary.PrintString` (`KismetStringLibrary.BuildString_Int` "" "Quantity available: " (`local.L-QuantityIn`)) true true (struct :`G` 1.0 :`B` 0.148792 :`A` 1.0) 5.0)
    (`KismetSystemLibrary.PrintString` (`KismetStringLibrary.BuildString_Int` "" "Index to check: " (`local.L-Index`)) true true (struct :`G` 1.0 :`B` 0.14996 :`A` 1.0) 5.0)
    ;[1 1 1] Increment through map and check if key is occupied
    (`|ExecutionSequence`
      (:`then_0`
        (set `local.L-Remaining` _remaining)
        (if _returnvalue
          (`KismetSystemLibrary.PrintString` "branch 1 then" true true (struct :`G` 0.66 :`B` 1.0 :`A` 1.0) 5.0)
          ;[1 1 1] Check if same item found
          (if (== (`.DataAssets_5_7B5C6FD74B67BC9FE76869B6F1902922` (break `/Game/Stewart2/Inventory/Items/ST_Inventory` (`BlueprintMapLibrary.Map_Find` (`self.Inventory`) (`local.L-Index`)))) (`local.L-DataAssetIn`))
            (`KismetSystemLibrary.PrintString` "branch 2 then" true true (struct :`G` 0.66 :`B` 1.0 :`A` 1.0) 5.0)
            (set `local.L-FoundSameItem` true)
            (else
              (`KismetSystemLibrary.PrintString` "branch 2 else" true true (struct :`G` 0.66 :`B` 1.0 :`A` 1.0) 5.0)))
          (else
            (`KismetSystemLibrary.PrintString` "branch 1 else" true true (struct :`G` 0.66 :`B` 1.0 :`A` 1.0) 5.0)
            (bind _output_get (set `local.L-Remaining` _remaining))
            (if (== _output_get -1)
              (`KismetSystemLibrary.PrintString` "branch 3 then" true true (struct :`G` 0.66 :`B` 1.0 :`A` 1.0) 5.0)
              ;[1 1 1] Key is completely empty?
              (if (== -1 (`local.L-EmptyKey`))
                (`KismetSystemLibrary.PrintString` "branch 4 then" true true (struct :`G` 0.66 :`B` 1.0 :`A` 1.0) 5.0)
                (set `local.L-EmptyKey` (`local.L-Index`))
                ;[0 1 0.9099] again, thinking of adding as soon as it finds an empty
                (`KismetSystemLibrary.PrintString` "added in inv" true true (struct :`G` 0.66 :`B` 1.0 :`A` 1.0) 5.0)
                (`BlueprintMapLibrary.Map_Add` (`self.Inventory`) (`local.L-EmptyKey`) (make `/Game/Stewart2/Inventory/Items/ST_Inventory` _l_quantityin (`local.L-DataAssetIn`)))
                (`KismetSystemLibrary.PrintString` (`KismetStringLibrary.BuildString_Int` "" "New entry with  :" _l_quantityin) true true (struct :`R` 0.879622 :`B` 0.386429 :`A` 1.0) 5.0)
                (return true)
                (else
                  (`KismetSystemLibrary.PrintString` "branch 4 else" true true (struct :`G` 0.66 :`B` 1.0 :`A` 1.0) 5.0)))
              (else
                (`KismetSystemLibrary.PrintString` "branch 3 else" true true (struct :`G` 0.66 :`B` 1.0 :`A` 1.0) 5.0)
                ;[1 1 1] If the same item in key then...
                (if (== (`.DataAssets_5_7B5C6FD74B67BC9FE76869B6F1902922` (break `/Game/Stewart2/Inventory/Items/ST_Inventory` _value)) (`local.L-DataAssetIn`))
                  (`KismetSystemLibrary.PrintString` "branch 5 then" true true (struct :`G` 0.66 :`B` 1.0 :`A` 1.0) 5.0)
                  ;[1 1 1] add to key with qty in clamped to max
                  (`BlueprintMapLibrary.Map_Add` (`self.Inventory`) (`local.L-Index`) (make `/Game/Stewart2/Inventory/Items/ST_Inventory` (+ (`KismetMathLibrary.Clamp` (`local.L-QuantityIn`) 0 (`local.L-Remaining`)) (break `/Game/Stewart2/Inventory/Items/ST_Inventory` _value)) (`local.L-DataAssetIn`)))
                  (`KismetSystemLibrary.PrintString` (`KismetStringLibrary.BuildString_Int` "" "Updated entry to:" (break `/Game/Stewart2/Inventory/Items/ST_Inventory` (`BlueprintMapLibrary.Map_Find` (`self.Inventory`) (`local.L-Index`)))) true true (struct :`R` 0.791298 :`B` 0.346704 :`A` 1.0) 5.0)
                  ;[1 1 1] And reduce qty in but clamped to 0
                  (set `local.L-QuantityIn` (`KismetMathLibrary.Clamp` _returnvalue_2 0 _returnvalue_2))
                  (set `local.L-FoundSameItem` true)
                  (else
                    (`KismetSystemLibrary.PrintString` "branch 5 else" true true (struct :`G` 0.66 :`B` 1.0 :`A` 1.0) 5.0))))))))
      (:`then_1`
        (`KismetSystemLibrary.PrintString` (`KismetStringLibrary.BuildString_Int` "" "Completed index: " (`local.L-Index`)) true true (struct :`R` 1.0 :`A` 1.0) 5.0)
        (`/Engine/EditorBlueprintResources/StandardMacros.IncrementInt` (`local.L-Index`)))))
  ;[0 1 0.919] if we add during the body, just report complete?
  (`KismetSystemLibrary.PrintString` (`KismetStringLibrary.BuildString_Int` "" "While loop completed at index: " (`local.L-Index`)) true true (struct :`R` 1.0 :`A` 1.0) 5.0)
  ;[1 1 1] If consumed to existing key destroy actor
  (if (== (`local.L-QuantityIn`) 0)
    (`KismetSystemLibrary.PrintString` "branch 6 then" true true (struct :`G` 0.66 :`B` 1.0 :`A` 1.0) 5.0)
    (return true)
    (else
      (`KismetSystemLibrary.PrintString` "branch 6 else" true true (struct :`G` 0.66 :`B` 1.0 :`A` 1.0) 5.0)
      ;[1 0.564 0] Does this add a quanity to an object that doent allow duplicates?
      (if (and (not (`self.AllowDuplicates`)) (`local.L-FoundSameItem`))
        (`KismetSystemLibrary.PrintString` "branch 7 then" true true (struct :`G` 0.66 :`B` 1.0 :`A` 1.0) 5.0)
        (`/Game/Stewart2/Inventory/Items/A_Item.ModifyQuantity` (`local.Item`) (`local.L-QuantityIn`))
        (return false)
        (else
          (`KismetSystemLibrary.PrintString` "branch 7 else" true true (struct :`G` 0.66 :`B` 1.0 :`A` 1.0) 5.0)
          ;[1 1 1] Add item in new key
          (if (!= (`local.L-EmptyKey`) 0)
            (`KismetSystemLibrary.PrintString` "branch 8 then" true true (struct :`G` 0.66 :`B` 1.0 :`A` 1.0) 5.0)
            (`KismetSystemLibrary.PrintString` (`KismetStringLibrary.BuildString_Int` "" "Quantity  :" (break `/Game/Stewart2/Inventory/Items/ST_Inventory` (`BlueprintMapLibrary.Map_Find` (`self.Inventory`) (`local.L-Index`)))) true true (struct :`R` 1.0 :`G` 0.857893 :`B` 0.036924 :`A` 1.0) 5.0)
            (`BlueprintMapLibrary.Map_Add` (`self.Inventory`) (`local.L-EmptyKey`) (make `/Game/Stewart2/Inventory/Items/ST_Inventory` (`local.L-QuantityIn`) (`local.L-DataAssetIn`)))
            (`KismetSystemLibrary.PrintString` (`KismetStringLibrary.BuildString_Int` "" "Quantity  :" (break `/Game/Stewart2/Inventory/Items/ST_Inventory` (`BlueprintMapLibrary.Map_Find` (`self.Inventory`) (`local.L-Index`)))) true true (struct :`R` 1.0 :`G` 0.857893 :`B` 0.036924 :`A` 1.0) 5.0)
            (return true)
            (else
              (`KismetSystemLibrary.PrintString` "branch 8 else" true true (struct :`G` 0.66 :`B` 1.0 :`A` 1.0) 5.0)
              (return false))))))))