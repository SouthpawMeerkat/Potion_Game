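; BP_SigilPlate is a drawable sigil plate for a timed potion-making step, where tracing speed sets potion quality.
; DrawBrush paints a brush material onto a runtime render target that textures the plate.
; Points removes hit key points gathered from the Sphere hierarchy; the last one stops the game mode's timer.
; OutcomeCalculator then grades elapsed time, has the game mode create the potion, toggles the wand's hold component and destroys the plate.
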(event `self.ReceiveBeginPlay`
  (bind _sphere (`self.Sphere`))
  (`|ExecutionSequence`
    (:`then_0`
      (bind _returnvalue (`KismetRenderingLibrary.CreateRenderTarget2D` 512 512))
      (bind _output_get (set `self.RenderTarget` _returnvalue))
      (`KismetRenderingLibrary.ClearRenderTarget2D` _output_get (struct :`R` 0.15625 :`G` 0.031488 :`B` 0.001756 :`A` 1.0)))
    (:`then_1`
      (bind _returnvalue_2 (`KismetMaterialLibrary.CreateDynamicMaterialInstance` "/Game/Assets/Materials/M_SigilPlate.M_SigilPlate"))
      (`MaterialInstanceDynamic.SetTextureParameterValue` _returnvalue_2 "SigilBasePlate" (`self.RenderTarget`))
      (`PrimitiveComponent.SetMaterial` (`self.Cylinder`) 0 _returnvalue_2))
    (:`then_2`
      (bind _returnvalue_3 (`KismetMaterialLibrary.CreateDynamicMaterialInstance` "/Game/Assets/Materials/M_Drawn.M_Drawn"))
      (set `self.DrawMat` _returnvalue_3))
    (:`then_3`
      (bind _output_get_2 (set `self.KeyPoints` (`SceneComponent.GetChildrenComponents` _sphere false)))
      (`KismetArrayLibrary.Array_AddUnique` _output_get_2 _sphere))))

(fn `DrawBrush`
  (params (BrushTexture :type "Texture2D Object Reference") (BrushSize :type "Float (double-precision)") (DrawLocation :type "Vector2D Structure"))
  (bind _brushsize (`local.BrushSize`))
  (`|ExecutionSequence`
    (:`then_0`
      (`MaterialInstanceDynamic.SetTextureParameterValue` (`self.DrawMat`) "BrushTexture" BrushTexture))
    (:`then_1`
      (bind (_canvas _size _context) (`KismetRenderingLibrary.BeginDrawCanvasToRenderTarget` (`self.RenderTarget`)))
      (`Canvas.K2_DrawMaterial` _canvas (`self.DrawMat`) (- (* _size (`local.DrawLocation`)) (/ _brushsize 2.0)) (`KismetMathLibrary.MakeVector2D` _brushsize _brushsize) (0.0 0.0) (1.0 1.0) 0.0 (0.5 0.5))
      (`KismetRenderingLibrary.EndDrawCanvasToRenderTarget` _context))))

(fn `outcomeCalculator`
  (params (TimeElpased :type "Float (double-precision)"))
  (`|ExecutionSequence`
    (:`then_0`
      (if (<= TimeElpased (`self.HighestGoodTime`))
        (if (>= TimeElpased (`self.LowestGoodTime`))
          ;[1 1 1] Just right
          (set `self.OutputNumberKey` 1)
          (else
            ;[1 1 1] To fast
            (set `self.OutputNumberKey` 2)))
        (elif (== (`self.TimerLength`) TimeElpased)
          ;[1 1 1] To long, Missing Keypoints
          (set `self.OutputNumberKey` 4)
          (else
            ;[1 1 1] To Long, With All keypoints
            (set `self.OutputNumberKey` 3)))))
    (:`then_1`
      (`KismetSystemLibrary.PrintString` (`KismetStringLibrary.Conv_IntToString` (`self.OutputNumberKey`))))
    (:`then_2`
      ;[1 1 1] Create the potion
      (bind _asbp_game_mode_base (cast `/Game/Blueprints/BP_GameModeBase` (`GameplayStatics.GetGameMode`)))
      (set `/Game/Blueprints/BP_GameModeBase.PotionQuaility` (`self.OutputNumberKey`) _asbp_game_mode_base)
      (`/Game/Blueprints/BP_GameModeBase.CreatePotionActor` _asbp_game_mode_base)
      ;[1 1 1] drop the wand
      (if (not (`KismetSystemLibrary.IsValid` (`self.WandReference`)))
        (bind _returnvalue (`GameplayStatics.GetActorOfClass` "/Game/Blueprints/BP_Wand.BP_Wand_C"))
        (set `self.WandReference` _returnvalue))
      (`/Game/Blueprints/BPComponent_Hold.PickUpItem` (`/Game/Blueprints/BP_Wand.BPComponent_Hold` (`self.WandReference`))))
    (:`then_3`
      ;[1 1 1] destroy the plate
      (`self.K2_DestroyActor`))))

(fn `Points`
  (params (`Hit point` :type "SceneComponent Object Reference"))
  (`KismetArrayLibrary.Array_RemoveItem` (`self.KeyPoints`) `Hit point`)
  (`ActorComponent.K2_DestroyComponent` `Hit point`)
  (if (<= (`KismetArrayLibrary.Array_Length` (`self.KeyPoints`)) 0)
    (bind _asbp_game_mode_base (cast `/Game/Blueprints/BP_GameModeBase` (`GameplayStatics.GetGameMode`)))
    (`Widget.RemoveFromParent` (`/Game/Blueprints/BP_GameModeBase.SigilTimerWidgetRef` _asbp_game_mode_base))
    (set `/Game/Blueprints/BP_GameModeBase.bTimerRunning` false _asbp_game_mode_base)
    (bind _currentsigiltimerhandler (`/Game/Blueprints/BP_GameModeBase.CurrentSigilTimerHandler` _asbp_game_mode_base))
    (`self.outcomeCalculator` (`KismetSystemLibrary.K2_GetTimerElapsedTimeHandle` _currentsigiltimerhandler))
    (`KismetSystemLibrary.K2_ClearAndInvalidateTimerHandle` _currentsigiltimerhandler)
    (`self.K2_DestroyActor`)
    (bind _asbp_character_main (cast `/Game/Blueprints/BP_CharacterMain` (`GameplayStatics.GetPlayerPawn` 0)))
    (`GameplayStatics.PlaySound2D` null 1.0 1.0 0.0 null null)))

(fn `UserConstructionScript`)