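; Actor component that lets the player click its owning actor to inspect it up close, then return to the character.
; A click spawns a temporary camera attached to the owner, eases it to a holding offset, blends the view to it and disables movement.
; For the mortar and pestle it also shows that UI from the game mode.
; CloseWindow, also triggered by clicking again, undoes this, with flags and delays blocking click spam.
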(event `GetChar`
  ;[1 1 1] Cast to Character and store as CharacterRef
  (bind _outactors (`GameplayStatics.GetAllActorsOfClass` "/Game/Blueprints/BP_CharacterMain.BP_CharacterMain_C"))
  (set `self.CharacterRefHolding` (`|GetArrayItem` _outactors)))

(event `self.ReceiveBeginPlay`
  (`self.GetChar`)
  (add `Actor.OnClicked` (`self.GetOwner`) (delegate `onMouseClick`)))

(event `onMouseClick`
  (params (TouchedActor :type "Actor Object Reference") (ButtonPressed :type "Key Structure" :default "None"))
  (bind _characterrefholding (`self.CharacterRefHolding`))
  ;[1 1 1] Create new camera at object and move to it
  ;;[1 1 1] Only if not inspecting
  (if (`self.isHolding`)
    (`self.CloseWindow`)
    (else
      ;;[1 1 1] Lock out repeat use until activity is complete
      (if (not (`self.isClicked`))
        (set `self.isClicked` true)
        ;;[1 1 1] Create new camera on owning actor
        (bind _returnvalue (`|SpawnActorFromClass` "/Script/Engine.CameraActor" (`self.MeshLocRef`) "Undefined" "MultiplyWithRoot" null null))
        (bind _output_get (set `self.tempCamera` _returnvalue))
        (`SceneComponent.K2_AttachToComponent` (`Actor.RootComponent` _output_get) (`Actor.RootComponent` (`self.GetOwner`)) "None" "SnapToTarget" "SnapToTarget" "SnapToTarget" true)
        ;;;[1 1 1] fix aspect ratio
        (`CameraComponent.SetConstraintAspectRatio` (`CameraActor.CameraComponent` (`self.tempCamera`)) false)
        (`KismetSystemLibrary.MoveComponentTo` (`Actor.RootComponent` (`self.tempCamera`)) (`self.HoldingLocation`) (`self.HoldingRotation`) false false 0.3)
        (`PlayerController.SetViewTargetWithBlend` (`PlayerState.GetPlayerController` (`Pawn.PlayerState` _characterrefholding)) (`self.tempCamera`) 0.5 "VTBlend_Linear" 0.0 false)
        (`CharacterMovementComponent.DisableMovement` (`Character.CharacterMovement` _characterrefholding))
        (`|ExecutionSequence`
          (:`then_0`
            ;[1 1 1] Widget for Morta and Pestel
            (bind _returnvalue_2 (`GameplayStatics.GetActorOfClass` "/Game/Blueprints/BP_MorterAndPestel.BP_MorterAndPestel_C"))
            (if (== _returnvalue_2 TouchedActor)
              (bind _asbp_game_mode_base (cast `/Game/Blueprints/BP_GameModeBase` (`GameplayStatics.GetGameMode`)))
              (`UserWidget.AddToViewport` (`/Game/Blueprints/BP_GameModeBase.MortaAndPestle_UI_Ref` _asbp_game_mode_base) 0)))
          (:`then_1`
            ;;[1 1 1] Reduce spam
            (`KismetSystemLibrary.Delay` 0.3)
            (set `self.isHolding` true)
            (set `self.isClicked` false)))))))

(event `self.CloseWindow`
  (bind _characterrefholding (`self.CharacterRefHolding`))
  ;[1 1 1] Return to player
  (bind _asbp_game_mode_base (cast `/Game/Blueprints/BP_GameModeBase` (`GameplayStatics.GetGameMode`)))
  (`Widget.RemoveFromParent` (`/Game/Blueprints/BP_GameModeBase.MortaAndPestle_UI_Ref` _asbp_game_mode_base))
  ;;[1 1 1] Only if inspecting
  (if (`self.isHolding`)
    (if (not (`self.isClicked`))
      (set `self.isClicked` true)
      ;;[1 1 1] Return camera to player
      (`PlayerController.SetViewTargetWithBlend` (`PlayerState.GetPlayerController` (`Pawn.PlayerState` (`self.CharacterRefHolding`))) _characterrefholding 0.5 "VTBlend_Linear" 0.0 false)
      (`CharacterMovementComponent.SetMovementMode` (`Character.CharacterMovement` _characterrefholding) "MOVE_Walking" 0)
      (`KismetSystemLibrary.Delay` 0.6)
      (`Actor.K2_DestroyActor` (`self.tempCamera`))
      ;;[1 1 1] Reduce spam
      (`KismetSystemLibrary.Delay` 0.3)
      (set `self.isHolding` false)
      (set `self.isClicked` false))))