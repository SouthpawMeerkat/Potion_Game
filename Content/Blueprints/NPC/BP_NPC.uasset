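; Customer NPC that walks a spline, stops at stop points to request a random potion, and is scored on the potion it receives.
; A random sprite and potion are picked on BeginPlay, and clicks show data-table-assembled dialogue or repeat lines in the UI.
; A tick-driven gate handles movement, closing on matching stop points.
; QualityCalculator scores potion, sigil and quality, then resumes movement; the next overlap destroys the NPC and spawns another.
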(event `self.PaperSprite.OnComponentBeginOverlap`
  (params (OverlappedComponent :type "PrimitiveComponent Object Reference") (OtherActor :type "Actor Object Reference") (OtherComp :type "PrimitiveComponent Object Reference") (OtherBodyIndex :type Integer) (bFromSweep :type Boolean) (SweepResult :type "HitResult Structure (by ref)"))
  (bind _asbp_stop_point (cast `/Game/Blueprints/NPC/BP_StopPoint` OtherActor))
  (if (`self.bRecievedPotion`)
    (`self.K2_DestroyActor`)
    (bind _returnvalue (`GameplayStatics.GetActorOfClass` "/Game/Blueprints/NPC/BP_NPC_Spawner.BP_NPC_Spawner_C"))
    (`/Game/Blueprints/NPC/BP_NPC_Spawner.SpawnNPC` _returnvalue)
    (elif (== (`/Game/Blueprints/NPC/BP_StopPoint.StopKey` _asbp_stop_point) (`self.movement`))
      (`/Engine/EditorBlueprintResources/StandardMacros.IncrementInt` (`self.movement`)
        (:`  `
          (goto _label :!via `Close`))))))

(event `MoveAgain`
  (goto _label :!via `Open`))

(event `self.ReceiveTick`
  (params (DeltaSeconds :type "Float (single-precision)"))
  (`/Engine/EditorBlueprintResources/StandardMacros.Gate` false :!label _label
    (:`Exit`
      (bind _output_get (set `self.NPCPosition` (+ (* DeltaSeconds (`self.NPCSpeed`)) (`self.NPCPosition`))))
      (`SceneComponent.K2_SetWorldLocation` (`self.PaperSprite`) (`SplineComponent.GetLocationAtDistanceAlongSpline` (`self.Spline`) _output_get "World") false false))))

(event `self.ReceiveBeginPlay`
  (bind _asbp_game_mode_base (cast `/Game/Blueprints/BP_GameModeBase` (`GameplayStatics.GetGameMode`)))
  (set `self.GameModeRef` _asbp_game_mode_base)
  (set `self.bFirstClick` true)
  (`self.ChangeSprite`)
  (`self.SelectPotion`))

(event `self.PaperSprite.OnClicked`
  (params (TouchedComponent :type "PrimitiveComponent Object Reference") (ButtonPressed :type "Key Structure"))
  (bind _ui_npc_textref (`/Game/Blueprints/BP_GameModeBase.UI_NPC_TextRef` (`self.GameModeRef`)))
  (`/Engine/EditorBlueprintResources/StandardMacros.DoOnce` false :!label _label_2
    (:`Completed`
      (if (`self.bFirstClick`)
        (set `self.bFirstClick` false)
        (bind _npc_text (`self.SelectText`))
        (bind _delay_length (`/Game/Blueprints/UI/UI_NPC_Text.NPCSpeach` (`/Game/Blueprints/BP_GameModeBase.UI_NPC_TextRef` (`self.GameModeRef`)) "None" false (`self.CurrentSprite`) _npc_text))
        (`KismetSystemLibrary.Delay` _delay_length)
        (else
          (bind _returnvalue (`DataTableFunctionLibrary.GetDataTableColumnAsString` "/Game/DataTable/NPCDataTables/RandomCustomers/DT_RepeatText.DT_RepeatText" "PossibleSpeak"))
          (bind _outitem (`KismetArrayLibrary.Array_Random` _returnvalue))
          (switch `string` _outitem
            (:`Default`
              (bind _delay_length_2 (`/Game/Blueprints/UI/UI_NPC_Text.NPCSpeach` _ui_npc_textref "None" false (`self.CurrentSprite`) (`KismetStringLibrary.Concat_StrStr` _outitem (`self.RequestedPotion`))))
              (`KismetSystemLibrary.Delay` _delay_length_2))
            (:`, it cant be that hard.`
              (bind _delay_length_3 (`/Game/Blueprints/UI/UI_NPC_Text.NPCSpeach` (`/Game/Blueprints/BP_GameModeBase.UI_NPC_TextRef` (`self.GameModeRef`)) "None" false (`self.CurrentSprite`) (`KismetStringLibrary.Concat_StrStr` (`self.RequestedPotion`) _outitem)))
              (`KismetSystemLibrary.Delay` _delay_length_3)))))
      (set `Widget.Visibility` "Hidden" (`/Game/Blueprints/UI/UI_NPC_Text.CanvasPanel_79` _ui_npc_textref))
      (set `/Game/Blueprints/BP_GameModeBase.ArdenTime` true (`self.GameModeRef`))
      (goto _label_2 :!via `Reset`))))

(fn `ChangeSprite`
  (bind _outrownames (`DataTableFunctionLibrary.GetDataTableRowNames` "/Game/DataTable/NPCDataTables/RandomCustomers/DT_NPC_Sprites.DT_NPC_Sprites"))
  (bind _returnvalue (`|GetDataTableRow` "/Game/DataTable/NPCDataTables/RandomCustomers/DT_NPC_Sprites.DT_NPC_Sprites" (`KismetArrayLibrary.Array_Random` _outrownames))
    (:`then`
      (bind _output_get (set `self.CurrentSprite` (break `/Game/DataTable/NPCDataTables/RandomCustomers/DS_NPC_Sprites` _returnvalue)))
      (`PaperSpriteComponent.SetSprite` (`self.PaperSprite`) _output_get))))

(fn `QualityCalculator`
  (params (PotionName :type Name) (SigilName :type Name) (Quality :type Integer))
  (returns (FinalScore :type "Float (double-precision)"))
  (set `self.FinalScore` 0.0)
  (`|ExecutionSequence`
    (:`then_0`
      (if (`KismetStringLibrary.EqualEqual_StrStr` (`KismetStringLibrary.Conv_NameToString` (`local.SigilName`)) (`self.Needed Sigil`))
        (set `self.FinalScore` (+ (`self.FinalScore`) 50.0))
        (else
          (set `self.FinalScore` (+ (`self.FinalScore`) 25.0)))))
    (:`then_1`
      (switch `int` (`local.Quality`)
        (:`1`
          (set `self.FinalScore` (* (`self.FinalScore`) 1.5)))
        (:`2`
          (set `self.FinalScore` (* (`self.FinalScore`) 1.0)))
        (:`3`
          (set `self.FinalScore` (* (`self.FinalScore`) 0.75)))
        (:`4`
          (set `self.FinalScore` (* (`self.FinalScore`) 0.5)))))
    (:`then_2`
      (if (`KismetStringLibrary.EqualEqual_StrStr` (`KismetStringLibrary.Conv_NameToString` (`local.PotionName`)) (`self.RequestedPotion`))
        (set `self.FinalScore` (* (`self.FinalScore`) 2.0))
        (else
          (set `self.FinalScore` (* (`self.FinalScore`) -1.0)))))
    (:`then_3`
      (set `self.bRecievedPotion` true)
      (`self.MoveAgain`)
      (return (`self.FinalScore`)))))

(fn `SelectPotion`
  (bind _outrownames (`DataTableFunctionLibrary.GetDataTableRowNames` "/Game/Blueprints/DataTable_Potions/DataTable_Potions_Truncated.DataTable_Potions_Truncated"))
  (bind _returnvalue (`|GetDataTableRow` "/Game/Blueprints/DataTable_Potions/DataTable_Potions_Truncated.DataTable_Potions_Truncated" (`KismetArrayLibrary.Array_Random` _outrownames))
    (:`then`
      (set `self.RequestedPotion` (`.PotionName_9_FAEB207F499DAFD4FD7C8A87D502CC84` (break `/Game/Blueprints/DataTable_Potions/STRUCT_Potion` _returnvalue)))
      (set `self.Needed Sigil` (`|GetEnumeratorNameAsString` (`.Sigil_28_E6EEC3084A8C80E8CC5D6C8560D374A6` (break `/Game/Blueprints/DataTable_Potions/STRUCT_Potion` _returnvalue)))))))

(fn `SelectText`
  (returns (`NPC Text` :type String))
  (`|ExecutionSequence`
    (:`then_0`
      (bind _returnvalue (`DataTableFunctionLibrary.GetDataTableColumnAsString` "/Game/DataTable/NPCDataTables/RandomCustomers/DT_TextGreeting.DT_TextGreeting" "PossibleSpeak"))
      (set `self.Text` (`KismetArrayLibrary.Array_Random` _returnvalue)))
    (:`then_1`
      (bind _returnvalue_2 (`DataTableFunctionLibrary.GetDataTableColumnAsString` "/Game/DataTable/NPCDataTables/RandomCustomers/DT_TextAsk.DT_TextAsk" "PossibleSpeak"))
      (set `self.Text` (`KismetStringLibrary.Concat_StrStr` (`self.Text`) (`KismetStringLibrary.Concat_StrStr` (`KismetArrayLibrary.Array_Random` _returnvalue_2) (`self.RequestedPotion`)))))
    (:`then_2`
      (bind _returnvalue_3 (`DataTableFunctionLibrary.GetDataTableColumnAsString` "/Game/DataTable/NPCDataTables/RandomCustomers/DT_TextFinish.DT_TextFinish" "PossibleSpeak"))
      (set `self.Text` (`KismetStringLibrary.Concat_StrStr` (`self.Text`) (`KismetArrayLibrary.Array_Random` _returnvalue_3))))
    (:`then_3`
      (return (`self.Text`)))))

(fn `UserConstructionScript`)