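; NPC spawner that places either a story NPC or a generic BP_NPC at its Sphere component's transform.
; It spawns once on BeginPlay after building the story class array, currently only Carrie, and again whenever SpawnNPC is called.
; A weighted roll on StoryChance picks the type: each generic spawn, scaled down after creation, raises the chance, and a story spawn resets it to zero.
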(event `self.ReceiveBeginPlay`
  (`self.CreateNPCArray`)
  (if (`KismetMathLibrary.RandomBoolWithWeight` (`self.StoryChance`)) :!label _label
    (`|SpawnActorFromClass` (`KismetArrayLibrary.Array_Random` (`self.StoryNPCs`)) (`SceneComponent.K2_GetComponentToWorld` (`self.Sphere`)) "AdjustIfPossibleButAlwaysSpawn" "MultiplyWithRoot" null null)
    (set `self.StoryChance` 0.0)
    (else
      (bind _returnvalue (`|SpawnActorFromClass` "/Game/Blueprints/NPC/BP_NPC.BP_NPC_C" (`SceneComponent.K2_GetComponentToWorld` (`self.Sphere`)) "AdjustIfPossibleButAlwaysSpawn" "MultiplyWithRoot" null null))
      (`self.SetActorScale3D` _returnvalue (0.2 0.2 0.2))
      (set `self.StoryChance` (+ (`self.StoryChance`) 0.33)))))

(event `SpawnNPC`
  (goto _label))

(fn `CreateNPCArray`
  (`KismetArrayLibrary.Array_AddUnique` (`self.StoryNPCs`) "/Game/Blueprints/NPC/Carrie/BP_Story_NPC_Carrie.BP_Story_NPC_Carrie_C"))

(fn `UserConstructionScript`)