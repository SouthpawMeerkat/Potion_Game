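; Story customer NPC, the Count, who walks a spline to a stop point, talks when clicked and takes a crafted potion.
; Dialogue comes from data tables keyed by game instance progression and earlier outcomes, with random wait lines on repeat clicks.
; Delivered potions are rated Good, Neutral or Bad and saved as story outcomes.
; Afterwards he moves on, destroys himself at a stop point and has the spawner send another NPC.
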(event `self.PaperSprite.OnComponentBeginOverlap`
  (params (OverlappedComponent :type "PrimitiveComponent Object Reference") (OtherActor :type "Actor Object Reference") (OtherComp :type "PrimitiveComponent Object Reference") (OtherBodyIndex :type Integer) (bFromSweep :type Boolean) (SweepResult :type "HitResult Structure (by ref)"))
  (bind _asbp_stop_point (cast `/Game/Blueprints/NPC/BP_StopPoint` OtherActor))
  (if (`self.bRecievedPotion`)
    (`self.K2_DestroyActor`)
    (bind _returnvalue (`GameplayStatics.GetActorOfClass` "/Game/Blueprints/NPC/BP_NPC_Spawner.BP_NPC_Spawner_C"))
    (`/Game/Blueprints/NPC/BP_NPC_Spawner.SpawnNPC` _returnvalue)
    (elif (== (`/Game/Blueprints/NPC/BP_StopPoint.StopKey` _asbp_stop_point) (`self.movement`))
      (`/Engine/EditorBlueprintResources/StandardMacros.IncrementInt` (`self.movement`)
        (:`  `
          (goto _label :!via `Close`))))))

(event `Move again`
  (goto _label :!via `Open`))

(event `self.ReceiveTick`
  (params (DeltaSeconds :type "Float (single-precision)"))
  (`/Engine/EditorBlueprintResources/StandardMacros.Gate` false :!label _label
    (:`Exit`
      (bind _output_get (set `self.NPCPosition` (+ (* DeltaSeconds (`self.NPCSpeed`)) (`self.NPCPosition`))))
      (`SceneComponent.K2_SetWorldLocation` (`self.PaperSprite`) (`SplineComponent.GetLocationAtDistanceAlongSpline` (`self.Spline`) _output_get "World") false false))))

(event `self.ReceiveBeginPlay`
  (bind _asbp_game_mode_base (cast `/Game/Blueprints/BP_GameModeBase` (`GameplayStatics.GetGameMode`)))
  (set `self.As BP Game Mode Base` _asbp_game_mode_base)
  (bind _asbp_game_instance (cast `/Game/Blueprints/BP_GameInstance` (`GameplayStatics.GetGameInstance`)))
  (set `self.As BP Game Instance` _asbp_game_instance))

(event `self.ReceiveActorOnClicked`
  (params (ButtonPressed :type "Key Structure"))
  (if (not (`self.bRecievedPotion`))
    (`/Engine/EditorBlueprintResources/StandardMacros.DoOnce` false :!label _label_2
      (:`Completed`
        (if (`self.bFirstClick`)
          (set `self.bFirstClick` false)
          (`self.SelectText` :!label _label_3)
          (bind _delay_length (`/Game/Blueprints/UI/UI_NPC_Text.NPCSpeach` (`/Game/Blueprints/BP_GameModeBase.UI_NPC_TextRef` (`self.As BP Game Mode Base`)) "None" false (`PaperSpriteComponent.GetSprite` (`self.PaperSprite`)) (`self.Text`)))
          (`KismetSystemLibrary.Delay` _delay_length)
          (elif (`KismetMathLibrary.RandomBoolWithWeight` (`self.Rerequest`))
            (set `self.Rerequest` 0.0)
            (goto _label_3)
            (else
              (set `self.Rerequest` 1.0)
              (bind _outrownames (`DataTableFunctionLibrary.GetDataTableRowNames` "/Game/DataTable/NPCDataTables/Story_NPC/DT_TheCount_Wait_Text.DT_TheCount_Wait_Text"))
              (bind _returnvalue (`|GetDataTableRow` "/Game/DataTable/NPCDataTables/Story_NPC/DT_TheCount_Wait_Text.DT_TheCount_Wait_Text" (`KismetArrayLibrary.Array_Random` _outrownames))
                (:`then`
                  (bind _delay_length_2 (`/Game/Blueprints/UI/UI_NPC_Text.NPCSpeach` (`/Game/Blueprints/BP_GameModeBase.UI_NPC_TextRef` (`self.As BP Game Mode Base`)) "None" false (`PaperSpriteComponent.GetSprite` (`self.PaperSprite`)) (break `/Game/DataTable/NPCDataTables/Story_NPC/DS_StoryNPC_Waiting_text` _returnvalue)))
                  (`KismetSystemLibrary.Delay` _delay_length_2))))))
        (set `Widget.Visibility` "Hidden" (`/Game/Blueprints/UI/UI_NPC_Text.CanvasPanel_79` (`/Game/Blueprints/BP_GameModeBase.UI_NPC_TextRef` (`self.As BP Game Mode Base`))))
        (if (`self.bFinal`)
          (`self.Move again `)
          (set `self.bRecievedPotion` true)
          (else
            (goto _label_2 :!via `Reset`)))))))

(event `self.Box.OnComponentBeginOverlap`
  (params (OverlappedComponent :type "PrimitiveComponent Object Reference") (OtherActor :type "Actor Object Reference") (OtherComp :type "PrimitiveComponent Object Reference") (OtherBodyIndex :type Integer) (bFromSweep :type Boolean) (SweepResult :type "HitResult Structure (by ref)"))
  (bind _asbp_crafted_potion (cast `/Game/Blueprints/BP_CraftedPotion` OtherActor))
  (`self.QualityCalculator` (`/Game/Blueprints/BP_CraftedPotion.Potion Name` _asbp_crafted_potion) (`/Game/Blueprints/BP_CraftedPotion.Chosen Sigil` _asbp_crafted_potion) (`/Game/Blueprints/BP_CraftedPotion.Sigil Quaility` _asbp_crafted_potion))
  (`/Game/Blueprints/InspectionManager/BPC_PickupObject.PickupObject` (`/Game/Blueprints/BP_CraftedPotion.BPC_PickupObject` _asbp_crafted_potion))
  (`self.K2_DestroyActor` _asbp_crafted_potion))

(fn `PotionChecker`
  (bind _outrownames (`DataTableFunctionLibrary.GetDataTableRowNames` "/Game/DataTable/NPCDataTables/Story_NPC/DT_TheCount_Potions.DT_TheCount_Potions"))
  (for _array_element _outrownames
    (bind _returnvalue (`|GetDataTableRow` "/Game/DataTable/NPCDataTables/Story_NPC/DT_TheCount_Potions.DT_TheCount_Potions" _array_element)
      (:`then`
        (if (== (`/Game/Blueprints/BP_GameInstance.TheCountProgression` (`self.As BP Game Instance`)) (`.Incounter_8_6E41D1684100E73663F21FB9FCA7DF99` (break `/Game/DataTable/NPCDataTables/Story_NPC/DS_Story_NPC_Potion` _returnvalue)))
          (`KismetArrayLibrary.Array_AddUnique` (`self.Potions Array`) _array_element))))))

(fn `QualityCalculator`
  (params (PotionName :type Name) (SigilName :type Name) (Quality :type Integer))
  (returns (OutCome :type String))
  (bind _as_bp_game_instance (`self.As BP Game Instance`))
  (for _array_element (`self.Potions Array`)
    (bind _returnvalue (`|GetDataTableRow` "/Game/DataTable/NPCDataTables/Story_NPC/DT_TheCount_Potions.DT_TheCount_Potions" _array_element)
      (:`then`
        (bind (_storypath _neededpotion) (break `/Game/DataTable/NPCDataTables/Story_NPC/DS_Story_NPC_Potion` _returnvalue))
        (if (`KismetStringLibrary.EqualEqual_StrStr` (`KismetStringLibrary.Conv_NameToString` PotionName) _neededpotion)
          (switch `string` _storypath
            (:`Good`
              ;[0.6139 1 0.4279] Good
              (set `self.OutCome` _storypath))
            (:`Neutral`
              ;[1 0.7843 0.3062] Neutral
              (set `self.OutCome` _storypath))
            (:`Bad`
              ;[1 0.06227 0.08216] Bad
              (set `self.OutCome` _storypath)))))))
  (if (`KismetStringLibrary.IsEmpty` (`self.OutCome`))
    (set `self.OutCome` "Bad"))
  (bind _result (`/Engine/EditorBlueprintResources/StandardMacros.IncrementInt` (`/Game/Blueprints/BP_GameInstance.TheCountProgression` _as_bp_game_instance))
    (:`  `
      (`BlueprintMapLibrary.Map_Add` (`/Game/Blueprints/BP_GameInstance.TheCountStoryOutcomes` _as_bp_game_instance) _result (`self.OutCome`))
      (`self.Move again `)
      (set `self.bRecievedPotion` true)
      (return (`self.OutCome`)))))

(fn `SelectText`
  (bind _outrownames (`DataTableFunctionLibrary.GetDataTableRowNames` "/Game/DataTable/NPCDataTables/Story_NPC/DT_TheCount_Text.DT_TheCount_Text"))
  (bind _returnvalue (`DataTableFunctionLibrary.GetDataTableColumnAsString` "/Game/DataTable/NPCDataTables/Story_NPC/DT_TheCount_Text.DT_TheCount_Text" "Incounter"))
  (for (_array_element _array_index) _returnvalue
    (if (`KismetStringLibrary.EqualEqual_StrStr` _array_element (`KismetStringLibrary.Conv_IntToString` (`/Game/Blueprints/BP_GameInstance.TheCountProgression` (`self.As BP Game Instance`))))
      (bind _returnvalue_2 (`|GetDataTableRow` "/Game/DataTable/NPCDataTables/Story_NPC/DT_TheCount_Text.DT_TheCount_Text" (`|GetArrayItem` _outrownames _array_index))
        (:`then`
          (bind (_storypath _text _incounter _bfinaltext) (break `/Game/DataTable/NPCDataTables/Story_NPC/DS_Story_NPC_Text` _returnvalue_2))
          (if (`KismetStringLibrary.EqualEqual_StrStr` (`BlueprintMapLibrary.Map_Find` (`/Game/Blueprints/BP_GameInstance.TheCountStoryOutcomes` (`self.As BP Game Instance`)) _incounter) _storypath)
            (set `self.Text` _text)
            (if _bfinaltext
              (set `self.bFinal` true))))))))

(fn `UserConstructionScript`)