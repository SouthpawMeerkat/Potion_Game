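; Story NPC Carrie, a potion customer who moves along a spline until a matching stop point closes her movement gate.
; Her progression and previous outcome in the GameInstance select branching data-table rows for click-triggered dialogue and the requested potion and sigil.
; QualityCalculator scores a potion by sigil, quality and name, then records a Good, Neutral or Bad outcome and advances her story.
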(event `self.PaperSprite.OnComponentBeginOverlap`
  (params (OverlappedComponent :type "PrimitiveComponent Object Reference") (OtherActor :type "Actor Object Reference") (OtherComp :type "PrimitiveComponent Object Reference") (OtherBodyIndex :type Integer) (bFromSweep :type Boolean) (SweepResult :type "HitResult Structure (by ref)"))
  (bind _asbp_stop_point (cast `/Game/Blueprints/NPC/BP_StopPoint` OtherActor))
  (if (== (`/Game/Blueprints/NPC/BP_StopPoint.StopKey` _asbp_stop_point) (`self.movement`))
    (`/Engine/EditorBlueprintResources/StandardMacros.IncrementInt` (`self.movement`)
      (:`  `
        (goto _label :!via `Close`)))))

(event `self.ReceiveTick`
  (params (DeltaSeconds :type "Float (single-precision)"))
  (`/Engine/EditorBlueprintResources/StandardMacros.Gate` false :!label _label
    (:`Exit`
      (bind _output_get (set `self.NPCPosition` (+ (* DeltaSeconds (`self.NPCSpeed`)) (`self.NPCPosition`))))
      (`SceneComponent.K2_SetWorldLocation` (`self.PaperSprite`) (`SplineComponent.GetLocationAtDistanceAlongSpline` (`self.Spline`) _output_get "World") false false))))

(event `self.ReceiveBeginPlay`
  (bind _asbp_game_mode_base (cast `/Game/Blueprints/BP_GameModeBase` (`GameplayStatics.GetGameMode`)))
  (set `self.As BP Game Mode Base` _asbp_game_mode_base)
  (bind _asbp_game_instance (cast `/Game/Blueprints/BP_GameInstance` (`GameplayStatics.GetGameInstance`)))
  (set `self.As BP Game Instance` _asbp_game_instance)
  (`self.PotionDataSetter`))

(event `self.ReceiveActorOnClicked`
  (params (ButtonPressed :type "Key Structure"))
  (`/Engine/EditorBlueprintResources/StandardMacros.DoOnce` false :!label _label_2
    (:`Completed`
      (if (`self.bFirstClick`)
        (set `self.bFirstClick` false))
      (`self.SelectText`)
      (bind _delay_length (`/Game/Blueprints/UI/UI_NPC_Text.NPCSpeach` (`/Game/Blueprints/BP_GameModeBase.UI_NPC_TextRef` (`self.As BP Game Mode Base`)) "None" false (`PaperSpriteComponent.GetSprite` (`self.PaperSprite`)) (`self.Text`)))
      (`KismetSystemLibrary.Delay` _delay_length)
      (set `Widget.Visibility` "Hidden" (`/Game/Blueprints/UI/UI_NPC_Text.CanvasPanel_79` (`/Game/Blueprints/BP_GameModeBase.UI_NPC_TextRef` (`self.As BP Game Mode Base`))))
      (goto _label_2 :!via `Reset`))))

(fn `PotionDataSetter`
  (bind _carrieprogression (`/Game/Blueprints/BP_GameInstance.CarrieProgression` (`self.As BP Game Instance`)))
  (bind _value (`BlueprintMapLibrary.Map_Find` (`/Game/Blueprints/BP_GameInstance.CarrieStoryOutcomes` (`self.As BP Game Instance`)) (- _carrieprogression 1)))
  (`|ExecutionSequence`
    (:`then_0`
      ;[0.3605 0.8697 1] Set Potion needed
      (switch `int` _carrieprogression
        (:`1`
          (bind _returnvalue (`|GetDataTableRow` "/Game/DataTable/NPCDataTables/Carrie/DT_Carrie_Potions.DT_Carrie_Potions" "FirstRequest")
            (:`then`
              (set `self.RequestedPotion` (`.NeededPotion_5_7E93D06C4D8A2CFD445C7AA72D4EAE1F` (break `/Game/DataTable/NPCDataTables/Carrie/DS_Carrie_Potions` _returnvalue))))))
        (:`2`
          (switch `string` _value
            (:`Good`
              (bind _returnvalue_2 (`|GetDataTableRow` "/Game/DataTable/NPCDataTables/Carrie/DT_Carrie_Potions.DT_Carrie_Potions" "SecondRequestA")
                (:`then`
                  (set `self.RequestedPotion` (`.NeededPotion_5_7E93D06C4D8A2CFD445C7AA72D4EAE1F` (break `/Game/DataTable/NPCDataTables/Carrie/DS_Carrie_Potions` _returnvalue_2))))))
            (:`Bad`
              (bind _returnvalue_3 (`|GetDataTableRow` "/Game/DataTable/NPCDataTables/Carrie/DT_Carrie_Potions.DT_Carrie_Potions" "SecondRequestB")
                (:`then`
                  (set `self.RequestedPotion` (`.NeededPotion_5_7E93D06C4D8A2CFD445C7AA72D4EAE1F` (break `/Game/DataTable/NPCDataTables/Carrie/DS_Carrie_Potions` _returnvalue_3))))))
            (:`Neutral`
              (bind _returnvalue_4 (`|GetDataTableRow` "/Game/DataTable/NPCDataTables/Carrie/DT_Carrie_Potions.DT_Carrie_Potions" "SecondRequestC")
                (:`then`
                  (set `self.RequestedPotion` (`.NeededPotion_5_7E93D06C4D8A2CFD445C7AA72D4EAE1F` (break `/Game/DataTable/NPCDataTables/Carrie/DS_Carrie_Potions` _returnvalue_4))))))))
        (:`3`
          (switch `string` _value
            (:`Good`
              (bind _returnvalue_5 (`|GetDataTableRow` "/Game/DataTable/NPCDataTables/Carrie/DT_Carrie_Potions.DT_Carrie_Potions" "ThirdRequestA")
                (:`then`
                  (set `self.RequestedPotion` (`.NeededPotion_5_7E93D06C4D8A2CFD445C7AA72D4EAE1F` (break `/Game/DataTable/NPCDataTables/Carrie/DS_Carrie_Potions` _returnvalue_5))))))
            (:`Bad`
              (bind _returnvalue_6 (`|GetDataTableRow` "/Game/DataTable/NPCDataTables/Carrie/DT_Carrie_Potions.DT_Carrie_Potions" "ThirdRequestB")
                (:`then`
                  (set `self.RequestedPotion` (`.NeededPotion_5_7E93D06C4D8A2CFD445C7AA72D4EAE1F` (break `/Game/DataTable/NPCDataTables/Carrie/DS_Carrie_Potions` _returnvalue_6))))))
            (:`Neutral`
              (bind _returnvalue_7 (`|GetDataTableRow` "/Game/DataTable/NPCDataTables/Carrie/DT_Carrie_Potions.DT_Carrie_Potions" "ThirdRequestC")
                (:`then`
                  (set `self.RequestedPotion` (`.NeededPotion_5_7E93D06C4D8A2CFD445C7AA72D4EAE1F` (break `/Game/DataTable/NPCDataTables/Carrie/DS_Carrie_Potions` _returnvalue_7))))))))))
    (:`then_1`
      ;[1 0.353 1] Set Sigil
      (bind _returnvalue_8 (`DataTableFunctionLibrary.GetDataTableColumnAsString` "/Game/Blueprints/DataTable_Potions/DataTable_Potions_Truncated.DataTable_Potions_Truncated" "PotionName"))
      (bind _returnvalue_9 (`|GetDataTableRow` "/Game/Blueprints/DataTable_Potions/DataTable_Potions_Truncated.DataTable_Potions_Truncated" (`KismetStringLibrary.Conv_StringToName` (`KismetStringLibrary.Conv_IntToString` (`KismetArrayLibrary.Array_Find` _returnvalue_8 (`self.RequestedPotion`)))))
        (:`then`
          (set `self.RequestedPotion` (`.PotionName_9_FAEB207F499DAFD4FD7C8A87D502CC84` (break `/Game/Blueprints/DataTable_Potions/STRUCT_Potion` _returnvalue_9)))
          (set `self.Needed Sigil` (`|GetEnumeratorNameAsString` (`.Sigil_28_E6EEC3084A8C80E8CC5D6C8560D374A6` (break `/Game/Blueprints/DataTable_Potions/STRUCT_Potion` _returnvalue_9)))))))))

(fn `QualityCalculator`
  (params (PotionName :type Name) (SigilName :type Name) (Quality :type Integer))
  (returns (FinalScore :type "Float (double-precision)"))
  (bind _finalscore (`self.FinalScore`))
  (bind _as_bp_game_instance (`self.As BP Game Instance`))
  (bind _carrieprogression (`/Game/Blueprints/BP_GameInstance.CarrieProgression` _as_bp_game_instance))
  (set `self.FinalScore` 0.0)
  (`|ExecutionSequence`
    (:`then_0`
      (if (`KismetStringLibrary.EqualEqual_StrStr` (`KismetStringLibrary.Conv_NameToString` (`local.SigilName`)) (`self.Needed Sigil`))
        (set `self.FinalScore` (+ (`self.FinalScore`) 50.0))
        (else
          (set `self.FinalScore` (+ (`self.FinalScore`) 25.0)))))
    (:`then_1`
      (switch `int` (`local.Quality`)
        (:`1`
          (set `self.FinalScore` (* (`self.FinalScore`) 1.5)))
        (:`2`
          (set `self.FinalScore` (* (`self.FinalScore`) 1.0)))
        (:`3`
          (set `self.FinalScore` (* (`self.FinalScore`) 0.75)))
        (:`4`
          (set `self.FinalScore` (* (`self.FinalScore`) 0.5)))))
    (:`then_2`
      (if (`KismetStringLibrary.EqualEqual_StrStr` (`KismetStringLibrary.Conv_NameToString` (`local.PotionName`)) (`self.RequestedPotion`))
        (set `self.FinalScore` (* (`self.FinalScore`) 2.0))
        (else
          (set `self.FinalScore` (* (`self.FinalScore`) -1.0)))))
    (:`then_3`
      (if (< _finalscore 0.0)
        ;[1 0.06227 0.08216] Negative Score
        (set `self.StoryOutcome` "Bad")
        (elif (<= _finalscore 50.0)
          ;[1 0.7843 0.3062] Low Score
          (set `self.StoryOutcome` "Neutral")
          (else
            ;[0.6139 1 0.4279] Good Score
            (set `self.StoryOutcome` "Good")))))
    (:`then_4`
      (`BlueprintMapLibrary.Map_Add` (`/Game/Blueprints/BP_GameInstance.CarrieStoryOutcomes` _as_bp_game_instance) _carrieprogression (`self.StoryOutcome`))
      (`/Engine/EditorBlueprintResources/StandardMacros.IncrementInt` _carrieprogression
        (:`  `
          (return (`self.FinalScore`)))))))

(fn `SelectText`
  (bind _carrieprogression (`/Game/Blueprints/BP_GameInstance.CarrieProgression` (`self.As BP Game Instance`)))
  (bind _value (`BlueprintMapLibrary.Map_Find` (`/Game/Blueprints/BP_GameInstance.CarrieStoryOutcomes` (`self.As BP Game Instance`)) (- _carrieprogression 1)))
  (switch `int` _carrieprogression
    (:`1`
      (bind _returnvalue (`|GetDataTableRow` "/Game/DataTable/NPCDataTables/Carrie/DT_Carrie_Text.DT_Carrie_Text" "FirstRequest")
        (:`then`
          (set `self.Text` (`.Text_5_E786C6AA4B6703A3943345B816F1A5A4` (break `/Game/DataTable/NPCDataTables/Carrie/DS_Carrie_Text` _returnvalue))))))
    (:`2`
      (switch `string` _value
        (:`Good`
          (bind _returnvalue_2 (`|GetDataTableRow` "/Game/DataTable/NPCDataTables/Carrie/DT_Carrie_Text.DT_Carrie_Text" "SecondRequestA")
            (:`then`
              (set `self.Text` (`.Text_5_E786C6AA4B6703A3943345B816F1A5A4` (break `/Game/DataTable/NPCDataTables/Carrie/DS_Carrie_Text` _returnvalue_2))))))
        (:`Bad`
          (bind _returnvalue_3 (`|GetDataTableRow` "/Game/DataTable/NPCDataTables/Carrie/DT_Carrie_Text.DT_Carrie_Text" "SecondRequestB")
            (:`then`
              (set `self.Text` (`.Text_5_E786C6AA4B6703A3943345B816F1A5A4` (break `/Game/DataTable/NPCDataTables/Carrie/DS_Carrie_Text` _returnvalue_3))))))
        (:`Neutral`
          (bind _returnvalue_4 (`|GetDataTableRow` "/Game/DataTable/NPCDataTables/Carrie/DT_Carrie_Text.DT_Carrie_Text" "SecondRequestC")
            (:`then`
              (set `self.Text` (`.Text_5_E786C6AA4B6703A3943345B816F1A5A4` (break `/Game/DataTable/NPCDataTables/Carrie/DS_Carrie_Text` _returnvalue_4))))))))
    (:`3`
      (switch `string` _value
        (:`Good`
          (bind _returnvalue_5 (`|GetDataTableRow` "/Game/DataTable/NPCDataTables/Carrie/DT_Carrie_Text.DT_Carrie_Text" "ThirdRequestA")
            (:`then`
              (set `self.Text` (`.Text_5_E786C6AA4B6703A3943345B816F1A5A4` (break `/Game/DataTable/NPCDataTables/Carrie/DS_Carrie_Text` _returnvalue_5))))))
        (:`Bad`
          (bind _returnvalue_6 (`|GetDataTableRow` "/Game/DataTable/NPCDataTables/Carrie/DT_Carrie_Text.DT_Carrie_Text" "ThirdRequestB")
            (:`then`
              (set `self.Text` (`.Text_5_E786C6AA4B6703A3943345B816F1A5A4` (break `/Game/DataTable/NPCDataTables/Carrie/DS_Carrie_Text` _returnvalue_6))))))
        (:`Neutral`
          (bind _returnvalue_7 (`|GetDataTableRow` "/Game/DataTable/NPCDataTables/Carrie/DT_Carrie_Text.DT_Carrie_Text" "ThirdRequestC")
            (:`then`
              (set `self.Text` (`.Text_5_E786C6AA4B6703A3943345B816F1A5A4` (break `/Game/DataTable/NPCDataTables/Carrie/DS_Carrie_Text` _returnvalue_7))))))))))

(fn `UserConstructionScript`)