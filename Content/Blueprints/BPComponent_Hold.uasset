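; Actor component that lets the player pick up an object to inspect it in front of the camera, then put it back.
; PickUpItem saves the original transform, attaches the owner's root to the camera manager and eases it to the holding pose, or calls CloseWindow if already held.
; CloseWindow closes the game mode's sigil widget, detaches and restores the transform.
; Delayed flags block spam; the click handler is empty.
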(event `GetChar`
  ;[1 1 1] Cast to Character and store as CharacterRef
  (bind _outactors (`GameplayStatics.GetAllActorsOfClass` "/Game/Blueprints/BP_CharacterMain.BP_CharacterMain_C"))
  (set `self.CharacterRefHolding` (`|GetArrayItem` _outactors)))

(event `self.ReceiveBeginPlay`
  (`self.GetChar`)
  (add `Actor.OnClicked` (`self.GetOwner`) (delegate `onMouseClick`)))

(event `onMouseClick`
  (params (TouchedActor :type "Actor Object Reference") (ButtonPressed :type "Key Structure" :default "None"))
  ;[1 0 0.03278] disabled mouse clicking, call pick up item instead
)

(event `PickUpItem`
  (bind _returnvalue (`self.GetOwner`))
  (bind _rootcomponent (`Actor.RootComponent` _returnvalue))
  ;[1 1 1] Inspect Object
  (bind _asbp_game_mode_base (cast `/Game/Blueprints/BP_GameModeBase` (`GameplayStatics.GetGameMode`)))
  (set `self.As BP Game Mode Base` _asbp_game_mode_base)
  (`/Engine/EditorBlueprintResources/StandardMacros.IsValid` _rootcomponent
    (:`Is Valid`
      ;;[1 1 1] Only pick up if not holding something
      (if (`self.isHolding`)
        (`self.CloseWindow`)
        (else
          ;;[1 1 1] Lock out repeat use until activity is complete
          (if (not (`self.isClicked`))
            (set `self.isClicked` true)
            (`|ExecutionSequence`
              (:`then_0`
                ;;[1 1 1] Get original transform
                (`/Engine/EditorBlueprintResources/StandardMacros.DoOnce` false :!label _label
                  (:`Completed`
                    (set `self.MeshLocRef` (`Actor.GetTransform` _returnvalue)))))
              (:`then_1`
                (`SceneComponent.K2_AttachToComponent` _rootcomponent (`PlayerCameraManager.TransformComponent` (`GameplayStatics.GetPlayerCameraManager` 0)) "None" "KeepWorld" "KeepWorld" "KeepWorld" true)
                (`KismetSystemLibrary.MoveComponentTo` _rootcomponent (`self.HoldingLocation`) (`self.HoldingRotation`) false false 0.3)
                ;;[1 1 1] Reduce spam
                (`KismetSystemLibrary.Delay` 0.3)
                (set `self.isHolding` true)
                (set `self.isClicked` false)))))))
    (:`Is Not Valid`
      (`KismetSystemLibrary.PrintString` "Not Valid Object"))))

(event `self.CloseWindow`
  (bind _returnvalue (`self.GetOwner`))
  (bind (_meshlocref_location _meshlocref_rotation) (`KismetMathLibrary.BreakTransform` (`self.MeshLocRef`)))
  ;[1 1 1] CloseRuneInspect
  ;;[1 1 1] Only drop if holding something
  (if (`self.isHolding`)
    (`/Game/Blueprints/BP_GameModeBase.Sigil Widget Closer` (`self.As BP Game Mode Base`))
    (if (not (`self.isClicked`))
      (set `self.isClicked` true)
      (`Actor.K2_DetachFromActor` _returnvalue "KeepWorld" "KeepWorld" "KeepWorld")
      (`KismetSystemLibrary.MoveComponentTo` (`Actor.RootComponent` _returnvalue) _meshlocref_location _meshlocref_rotation)
      ;;[1 1 1] Reduce spam
      (`KismetSystemLibrary.Delay` 0.3)
      (set `self.isHolding` false)
      (set `self.isClicked` false)
      (goto _label :!via `Reset`))))