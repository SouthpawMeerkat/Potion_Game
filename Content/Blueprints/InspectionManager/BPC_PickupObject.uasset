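; Actor component that lets the player pick up and drop its owning object by clicking it.
; Pickup closes any active inspection, then grabs the static mesh with the character's PhysicsHandle, and Tick holds it at a set distance in front of the camera.
; BP_InspectionManager's interacting state decides between grab and drop, with a lockout flag guarding pickup.
; Meshes not simulating physics trigger a debug warning and have physics switched on.
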(event `self.ReceiveTick`
  (params (DeltaSeconds :type "Float (single-precision)"))
  (bind _physicshandle (`/Game/Blueprints/BP_CharacterMain.PhysicsHandle` (`self.CharacterMainRef`)))
  (bind _camera (`/Game/Blueprints/BP_CharacterMain.Camera` (`self.CharacterMainRef`)))
  (bind _returnvalue (`SceneComponent.K2_GetComponentRotation` _camera))
  ;[1 1 1] Update position of picked up item via player physics handle
  (if (`KismetSystemLibrary.IsValid` (`PhysicsHandleComponent.GetGrabbedComponent` (`/Game/Blueprints/BP_CharacterMain.PhysicsHandle` (`self.CharacterMainRef`))))
    (if (not (`/Game/Blueprints/InspectionManager/BP_InspectionManager.isInteracting` (`self.InspectionManagerRef`)))
      (`/Game/Blueprints/InspectionManager/BP_InspectionManager.isInteractingSwitcher` (`self.InspectionManagerRef`) true))
    (`PhysicsHandleComponent.SetTargetLocation` _physicshandle (+ (`SceneComponent.K2_GetComponentLocation` _camera) (* (`KismetMathLibrary.GetForwardVector` _returnvalue) (`self.HeldObjectDistanceFromViewport`))))
    (`PhysicsHandleComponent.SetTargetRotation` _physicshandle _returnvalue)))

(event `DropObject`
  (bind _returnvalue (`self.GetOwner` self))
  ;[1 1 1] Drop object that has physics
  (if (`self.HasPhysics`)
    (`PhysicsHandleComponent.ReleaseComponent` (`/Game/Blueprints/BP_CharacterMain.PhysicsHandle` (`self.CharacterMainRef`)))
    (else
      (`KismetSystemLibrary.PrintString` "Physics Missing Error!!" true true (struct :`R` 1.0 :`G` 0.014287 :`A` 1.0) 6.0)
      ;[1 1 1] Drop and turn on physics
      (`Actor.K2_DetachFromActor` _returnvalue "KeepWorld" "KeepWorld" "KeepWorld")
      (`PrimitiveComponent.SetSimulatePhysics` (`Actor.GetComponentByClass` _returnvalue "/Script/Engine.StaticMeshComponent") true)))
  (`/Game/Blueprints/InspectionManager/BP_InspectionManager.isInteractingSwitcher` (`self.InspectionManagerRef`) false))

(event `PickupObject`
  (bind _inspectionmanagerref (`self.InspectionManagerRef`))
  (bind _isinteracting (`/Game/Blueprints/InspectionManager/BP_InspectionManager.isInteracting` (`self.InspectionManagerRef`)))
  (bind _returnvalue (`Actor.GetComponentByClass` (`self.GetOwner` self) "/Script/Engine.StaticMeshComponent"))
  ;[1 1 1] Checks
  (if (`KismetSystemLibrary.IsValid` (`/Game/Blueprints/InspectionManager/BP_InspectionManager.CurrentInspectedActor` _inspectionmanagerref))
    (`/Game/Blueprints/InspectionManager/BP_InspectionManager.CloseInspection` _inspectionmanagerref)
    (`/Game/Blueprints/InspectionManager/BP_InspectionManager.isInteractingSwitcher` (`self.InspectionManagerRef`) false))
  (if (and (not (`self.Lockout`)) (not _isinteracting))
    (set `self.Lockout` true)
    (`/Game/Blueprints/InspectionManager/BP_InspectionManager.isInteractingSwitcher` (`self.InspectionManagerRef`) true)
    (`self.PhysicsCheck` self)
    (if (`self.HasPhysics`)
      ;[1 1 1] if it has physics
      (`PhysicsHandleComponent.GrabComponentAtLocationWithRotation` (`/Game/Blueprints/BP_CharacterMain.PhysicsHandle` (`self.CharacterMainRef`)) _returnvalue "None" (`SceneComponent.K2_GetComponentLocation` _returnvalue) (`SceneComponent.K2_GetComponentRotation` _returnvalue))
      (set `self.Lockout` false)
      (else
        (`KismetSystemLibrary.PrintString` "WARNING! - Object physics not set" true true (struct :`R` 1.0 :`G` 0.83254 :`A` 1.0) 5.0)
        (`PrimitiveComponent.SetSimulatePhysics` (`Actor.GetComponentByClass` (`self.GetOwner` self) "/Script/Engine.StaticMeshComponent") true)
        (set `self.Lockout` false)
        (`self.PickupObject`)))
    (elif _isinteracting
      (`self.DropObject` self))))

(event `self.ReceiveBeginPlay`
  ;[1 1 1] Init
  (bind _returnvalue (`GameplayStatics.GetActorOfClass` "/Game/Blueprints/BP_CharacterMain.BP_CharacterMain_C"))
  (set `self.CharacterMainRef` _returnvalue)
  (bind _returnvalue_2 (`GameplayStatics.GetActorOfClass` "/Game/Blueprints/InspectionManager/BP_InspectionManager.BP_InspectionManager_C"))
  (set `self.InspectionManagerRef` _returnvalue_2)
  (add `Actor.OnClicked` (`self.GetOwner` self) (delegate `you know`)))

(event `you know`
  (params (TouchedActor :type "Actor Object Reference") (ButtonPressed :type "Key Structure" :default "None"))
  ;[1 1 1] Init
  (`self.PickupObject` self))

(fn `PhysicsCheck`
  (bind _returnvalue (`Actor.GetComponentByClass` (`self.GetOwner`) "/Script/Engine.StaticMeshComponent"))
  (`/Engine/EditorBlueprintResources/StandardMacros.IsValid` _returnvalue
    (:`Is Valid`
      (set `self.HasPhysics` (`SceneComponent.IsSimulatingPhysics` _returnvalue "None")))
    (:`Is Not Valid`
      (`KismetSystemLibrary.PrintString` "No Static Mesh Found")))
  (return))

(fn `PhysicsOn`
  (bind _returnvalue (`Actor.GetComponentByClass` (`self.GetOwner`) "/Script/Engine.StaticMeshComponent"))
  (if (and (`self.HasPhysics`) (`KismetSystemLibrary.IsValid` _returnvalue))
    (set `self.HasPhysics` false)
    (`PrimitiveComponent.SetSimulatePhysics` _returnvalue true)
    (`PrimitiveComponent.SetCollisionEnabled` _returnvalue "QueryAndPhysics")))