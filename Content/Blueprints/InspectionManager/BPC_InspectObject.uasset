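; Actor component that makes its owning actor inspectable by mouse click, binding to the owner's OnClicked event at BeginPlay.
; A click only proceeds when the touched actor is the BP_Cauldron or BP_Compendium found in the level and BP_InspectionManager is not already interacting.
; It then passes the owner, its root component and a custom vector and rotator to the manager's InspectNewObject.
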(event `self.ReceiveBeginPlay`
  ;[1 1 1] mouse click event calls inspect actor
  (add `Actor.OnClicked` (`self.GetOwner` self) (delegate `onMouseClick`)))

(event `InspectActor`
  (params (TouchedActor :type "Actor Object Reference"))
  (bind _returnvalue (`self.GetOwner` self))
  ;[1 1 1] Pass parent details to inspections manager
  (bind _returnvalue_2 (`GameplayStatics.GetActorOfClass` "/Game/Blueprints/InspectionManager/BP_InspectionManager.BP_InspectionManager_C"))
  (`/Game/Blueprints/InspectionManager/BP_InspectionManager.InspectNewObject ` _returnvalue_2 _returnvalue (`self.CustomVector`) (`self.CustomRotator`) (`Actor.RootComponent` _returnvalue)))

(event `onMouseClick`
  (params (TouchedActor :type "Actor Object Reference") (ButtonPressed :type "Key Structure" :default "None"))
  ;[1 1 1] mouse click event calls inspect actor
  (bind _returnvalue (`GameplayStatics.GetActorOfClass` "/Game/Blueprints/InspectionManager/BP_InspectionManager.BP_InspectionManager_C"))
  (bind _returnvalue_2 (`GameplayStatics.GetActorOfClass` "/Game/Blueprints/BP_Cauldron.BP_Cauldron_C"))
  (bind _returnvalue_3 (`GameplayStatics.GetActorOfClass` "/Game/Blueprints/Compendium/BP_Compendium.BP_Compendium_C"))
  (if (or (== TouchedActor _returnvalue_3) (== TouchedActor _returnvalue_2))
    (if (not (`/Game/Blueprints/InspectionManager/BP_InspectionManager.isInteracting` _returnvalue))
      (`self.InspectActor` null))))