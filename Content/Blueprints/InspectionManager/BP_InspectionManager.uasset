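; BP_InspectionManager runs camera-based close-up inspection of world objects, entering and leaving an inspection view.
; InspectNewObject locks buttons and player movement, spawns a temporary camera, attaches it at the given relative transform and blends the view to it, destroying any previous camera.
; CloseInspection blends back to the character, restores walking and destroys the camera.
; An IsCameraMoving flag with delays blocks overlapping transitions, while IsInteracting tracks the inspection state.
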(event `InspectNewObject`
  (params (NewActor :type "Actor Object Reference") (NewVector :type "Vector Structure") (NewRotator :type "Rotator Structure") (NewRoot :type "SceneComponent Object Reference"))
  (bind _lastcamera (`self.lastCamera`))
  (bind _tempcamera (`self.tempCamera`))
  ;[1 1 1] Initialise Inspection
  (if (not (`self.isCameraMoving`))
    (`self.OnButtonsLocked`)
    (set `self.isCameraMoving` true)
    (set `self.NewInspectedActor` NewActor)
    (set `self.Target Relative Location` NewVector)
    (set `self.Target Relative Rotation` NewRotator)
    (set `self.New Root` NewRoot)
    ;[1 0.7888 0] Disable player movement
    (bind _returnvalue (`GameplayStatics.GetActorOfClass` "/Game/Blueprints/BP_CharacterMain.BP_CharacterMain_C"))
    (set `self.CharacterReference` _returnvalue)
    (`CharacterMovementComponent.DisableMovement` (`Character.CharacterMovement` _returnvalue))
    (if (not (`self.isInteracting`))
      (`/Game/Blueprints/BP_CharacterMain.LockCamera` _returnvalue true))
    ;[1 1 1] Spawn inspection camera (as required)
    (`/Engine/EditorBlueprintResources/StandardMacros.IsValid` _tempcamera
      (:`Is Valid`
        (set `self.lastCamera` _tempcamera))
      (:`Is Not Valid`
        _))
    (bind _returnvalue_2 (`|SpawnActorFromClass` "/Script/Engine.CameraActor" (`self.Spawn Transform`) "Undefined" "MultiplyWithRoot" (`self.NewInspectedActor`) null))
    (set `self.TempCamera` _returnvalue_2)
    (`CameraComponent.SetConstraintAspectRatio` (`CameraActor.CameraComponent` (`self.TempCamera`)) false)
    ;[1 1 1] Move camera to inspection site
    (`KismetSystemLibrary.MoveComponentTo` (`Actor.RootComponent` (`self.TempCamera`)) (`self.Target Relative Location`) (`self.Target Relative Rotation`) false false 0.3)
    (`SceneComponent.K2_AttachToComponent` (`Actor.RootComponent` (`self.tempCamera`)) (`self.New Root`) "None" "KeepRelative" "KeepRelative" "KeepRelative" true)
    (`PlayerController.SetViewTargetWithBlend` (`PlayerState.GetPlayerController` (`Pawn.PlayerState` (`self.CharacterReference`))) (`self.TempCamera`) 0.5 "VTBlend_Linear" 0.0 false)
    (`KismetSystemLibrary.Delay` 0.6)
    ;[1 1 1] Clean up and complete
    (`/Engine/EditorBlueprintResources/StandardMacros.IsValid` _lastcamera
      (:`Is Valid`
        (`self.K2_DestroyActor` _lastcamera))
      (:`Is Not Valid`
        _))
    (set `self.isCameraMoving` false)
    (`self.isInteractingSwitcher` true)
    (set `self.CurrentInspectedActor` (`self.NewInspectedActor`))))

(event `CloseInspection`
  (bind _characterreference (`self.CharacterReference`))
  (bind _tempcamera (`self.tempCamera`))
  ;[1 1 1] Initialise closing sequence
  (if (not (`self.isCameraMoving`))
    (set `self.isCameraMoving` true)
    (if (`self.isInteracting`)
      ;[1 1 1] return camera to player
      (`/Game/Blueprints/BP_CharacterMain.LockCamera` (`self.CharacterReference`) true))
    (`KismetSystemLibrary.Delay` 0.2)
    (`PlayerController.SetViewTargetWithBlend` (`PlayerState.GetPlayerController` (`Pawn.PlayerState` _characterreference)) _characterreference 0.5 "VTBlend_Linear" 0.0 false)
    (`/Game/Blueprints/BP_CharacterMain.LockCamera` (`self.CharacterReference`) false)
    ;[1 0.9873 0] Enable Movement
    (`CharacterMovementComponent.SetMovementMode` (`Character.CharacterMovement` (`self.CharacterReference`)) "MOVE_Walking" 0)
    (`self.isInteractingSwitcher` false)
    ;[1 1 1] Clean up and complete
    (if (`KismetSystemLibrary.IsValid` _tempcamera)
      (`self.K2_DestroyActor` _tempcamera))
    (`KismetSystemLibrary.Delay` 0.2)
    (set `self.isCameraMoving` false)
    (set `self.CurrentInspectedActor` null)))

(fn `isInteractingSwitcher`
  (params (`isInteracting?` :type Boolean))
  (bind _output_get (set `self.isInteracting` `isInteracting?`)))

(fn `UserConstructionScript`)