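; Player controller Blueprint with a prototype left-click trace under the mouse cursor, used only for debug printing.
; When IA_LeftClick completes, it runs a Visibility line trace from the deprojected mouse location and prints the hit result and actor name.
; The trace End is left unset, as the mouse direction multiply is unconnected.
; A game-only input mode setup that hides the cursor exists but never runs.
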(event `self.ReceiveBeginPlay`)

(event `EnhancedInput|/Game/Blueprints/Actions/IA_LeftClick`
  (params (ActionValue :type Boolean) (ElapsedSeconds :type "Float (double-precision)") (TriggeredSeconds :type "Float (double-precision)") (InputAction :type "InputAction Object Reference" :default "/Game/Blueprints/Actions/IA_LeftClick.IA_LeftClick"))
  (:`Completed`
    (bind (_outhit _returnvalue) (`KismetSystemLibrary.LineTraceSingle` (`self.DeprojectMousePositionToWorld`) (0.0 0.0 0.0) "TraceTypeQuery1"))
    (`KismetSystemLibrary.PrintString` (`KismetStringLibrary.Conv_BoolToString` _returnvalue))
    (`KismetSystemLibrary.PrintString` (`KismetSystemLibrary.GetDisplayName` (`.HitActor` (`GameplayStatics.BreakHitResult` _outhit))))))

(fn `UserConstructionScript`)