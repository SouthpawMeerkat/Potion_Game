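; BP_CraftedPotion is an actor representing a crafted potion, carrying its name, chosen sigil and sigil quality.
; The Creation function stores those three values and sets StaticMesh to None.
; Clicking the mesh prints the values, destroys the actor and closes inspection through BP_InspectionManager, found by class lookup.
; The click handling is marked as subject to change.
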(event `self.StaticMesh.OnClicked`
  (params (TouchedComponent :type "PrimitiveComponent Object Reference") (ButtonPressed :type "Key Structure"))
  ;[1 0 0] will be changed
  (`KismetSystemLibrary.PrintString` (`KismetStringLibrary.Conv_NameToString` (`self.Potion Name`)))
  (`KismetSystemLibrary.PrintString` (`KismetStringLibrary.Conv_NameToString` (`self.Chosen Sigil`)))
  (`KismetSystemLibrary.PrintString` (`KismetStringLibrary.Conv_IntToString` (`self.Sigil Quaility`)))
  (`self.K2_DestroyActor`)
  (bind _returnvalue (`GameplayStatics.GetActorOfClass` "/Game/Blueprints/InspectionManager/BP_InspectionManager.BP_InspectionManager_C"))
  (`/Game/Blueprints/InspectionManager/BP_InspectionManager.CloseInspection` _returnvalue))

(fn `Creation`
  (params (PotionName :type Name) (ChosenSigil :type Name) (SigilQuaility :type Integer))
  (set `self.Potion Name` PotionName)
  (set `self.Chosen Sigil` ChosenSigil)
  (set `self.Sigil Quaility` SigilQuaility)
  (set `self.StaticMesh` null))

(fn `UserConstructionScript`)