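; Game mode for a potion-crafting game, holding shared UI references, crafting logic and NPC Arden's timed random speech.
; BeginPlay creates the NPC text, sigil, mortar, crafting and rune widgets.
; Potion calculators narrow data-table rows by three ingredients, optionally rune colour first, iterating a copied array while removing mismatches.
; Sigils and crafted potions spawn at the cauldron; DrawingTimer re-fires itself to end sigil drawing and trigger the plate's outcome.
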(event `self.ReceiveBeginPlay`
  (`self.WidgetFunction`))

(event `self.ReceiveTick`
  (params (DeltaSeconds :type "Float (single-precision)"))
  (if (`self.bArdenTime`)
    ;[1 1 1] Random Arden Speak
    (`/Engine/EditorBlueprintResources/StandardMacros.DoOnce` false :!label _label
      (:`Completed`
        (`KismetSystemLibrary.Delay` (`KismetMathLibrary.RandomFloatInRange` 10.0 20.0))
        (bind _delay_length (`/Game/Blueprints/UI/UI_NPC_Text.NPCSpeach` (`self.UI_NPC_TextRef`) (`KismetStringLibrary.Conv_StringToName` (`KismetStringLibrary.Conv_IntToString` (`KismetMathLibrary.RandomInteger` 10))) true null ""))
        (`KismetSystemLibrary.Delay` _delay_length)
        (`Widget.SetVisibility` (`/Game/Blueprints/UI/UI_NPC_Text.CanvasPanel_79` (`self.UI_NPC_TextRef`)) "Hidden")
        (goto _label :!via `Reset`)))))

(event `Drawing Timer`
  ;[1 1 1] Timer Event for Sigils
  (bind _asbp_character_main (cast `/Game/Blueprints/BP_CharacterMain` (`GameplayStatics.GetPlayerPawn` 0)))
  (if (`self.bTimerRunning`)
    (`KismetSystemLibrary.PrintString` "timer ended")
    (bind _returnvalue (`GameplayStatics.GetActorOfClass` "/Game/Blueprints/SigilPlateFolder/BP_SigilPlate.BP_SigilPlate_C"))
    (bind _timerlength (`/Game/Blueprints/SigilPlateFolder/BP_SigilPlate.TimerLength` (stale _returnvalue_2)))
    (`/Game/Blueprints/SigilPlateFolder/BP_SigilPlate.outcomeCalculator` _returnvalue _timerlength)
    (set `self.bTimerRunning` false)
    (`Widget.RemoveFromParent` (`self.SigilTimerWidgetRef`))
    (else
      (bind _returnvalue_2 (`GameplayStatics.GetActorOfClass` "/Game/Blueprints/SigilPlateFolder/BP_SigilPlate.BP_SigilPlate_C"))
      (set `self.Timer Length` _timerlength)
      (bind _returnvalue_3 (`KismetSystemLibrary.K2_SetTimerDelegate` (delegate `Drawing Timer`) _timerlength false 1.0))
      (set `self.CurrentSigilTimerHandler` _returnvalue_3)
      (set `self.bTimerRunning` true)
      (`UserWidget.AddToViewport` (`self.SigilTimerWidgetRef`) 0))))

(fn `Change Sigil`
  (params (`Spawned Sigil` :type "Actor Class Reference") (ChosenSigil :type Name))
  ;[1 1 1] Spawns selected sigil infront of player (unless player is not facing the X axis, needs to be made relative to players looking)
  (set `self.ChosenSigil` ChosenSigil)
  (bind _returnvalue (`GameplayStatics.GetActorOfClass` "/Game/Blueprints/BP_Cauldron.BP_Cauldron_C"))
  (bind _returnvalue_2 (`SceneComponent.K2_GetComponentToWorld` (`/Game/Blueprints/BP_Cauldron.DefaultSceneRoot` _returnvalue)))
  (`|SpawnActorFromClass` `Spawned Sigil` (`KismetMathLibrary.MakeTransform` (+ (.location _returnvalue_2) (-75.0 0.0 150.0)) (`KismetMathLibrary.MakeRotator` (.roll (.rotation _returnvalue_2)) (+ (.pitch (.rotation _returnvalue_2)) 80.0) (.yaw (.rotation _returnvalue_2))) (0.5 0.5 0.5)) "Undefined" "MultiplyWithRoot" null null))

(fn `CreatePotionActor`
  (bind _returnvalue (`GameplayStatics.GetActorOfClass` "/Game/Blueprints/BP_Cauldron.BP_Cauldron_C"))
  (bind _returnvalue_2 (`|SpawnActorFromClass` "/Game/Blueprints/BP_CraftedPotion.BP_CraftedPotion_C" (`SceneComponent.K2_GetComponentToWorld` (`/Game/Blueprints/BP_Cauldron.DefaultSceneRoot` _returnvalue)) "Undefined" "MultiplyWithRoot" null null))
  (`/Game/Blueprints/BP_CraftedPotion.Creation` _returnvalue_2 (`self.CurrentlyCrafting`) (`self.ChosenSigil`) (`self.PotionQuaility`))
  ;[1 0.7456 0] You want to pick up and hold the potion?
  (if (not (`KismetSystemLibrary.IsValid` (`self.CraftedPotionRef`)))
    (bind _returnvalue_3 (`GameplayStatics.GetActorOfClass` "/Game/Blueprints/BP_CraftedPotion.BP_CraftedPotion_C"))
    (set `self.CraftedPotionRef` _returnvalue_3))
  (`/Game/Blueprints/BPComponent_Hold.onMouseClick` (`/Game/Blueprints/BP_CraftedPotion.BPComponent_Hold` (`self.CraftedPotionRef`)) null "None"))

(fn `PotionArray`
  (`KismetArrayLibrary.Array_Clear` (`self.PossiblePotionsIntermidant`))
  (for _array_element (`self.Possible Potions`)
    (`KismetArrayLibrary.Array_AddUnique` (`self.PossiblePotionsIntermidant`) _array_element)))

(fn `PotionCalculator`
  (returns (CurrentlyCrafting :type Name))
  (bind _selected2 (`self.Selected2`))
  (bind _selected3 (`self.Selected3`))
  (bind _selected1 (`self.Selected1`))
  (`KismetArrayLibrary.Array_Clear` (`self.Possible Potions`))
  (bind _outrownames (`DataTableFunctionLibrary.GetDataTableRowNames` "/Game/Blueprints/DataTable_Potions/DataTable_Potions_Truncated.DataTable_Potions_Truncated"))
  (for _array_element _outrownames
    (bind _returnvalue (`|GetDataTableRow` "/Game/Blueprints/DataTable_Potions/DataTable_Potions_Truncated.DataTable_Potions_Truncated" _array_element)
      (:`then`
        (if (`KismetStringLibrary.EqualEqual_StrStr` (`|GetEnumeratorNameAsString` (`.RuneColour_27_4A69C2B74D9679D58B5A0FA84962FB1D` (break `/Game/Blueprints/DataTable_Potions/STRUCT_Potion` _returnvalue))) (`self.SelectedRuneCombinationColour`))
          (`KismetArrayLibrary.Array_AddUnique` (`self.Possible Potions`) _array_element)))))
  (`self.PotionArray`)
  (if (!= (`KismetArrayLibrary.Array_Length` (`self.Possible Potions`)) 0)
    (for _array_element_2 (`self.PossiblePotionsIntermidant`)
      (bind _returnvalue_2 (`|GetDataTableRow` "/Game/Blueprints/DataTable_Potions/DataTable_Potions_Truncated.DataTable_Potions_Truncated" _array_element_2)
        (:`then`
          (if (`KismetStringLibrary.EqualEqual_StrStr` (`|GetEnumeratorNameAsString` (`.Ingredient1_29_80935F3448C1E0AB5282968C8D72B828` (break `/Game/Blueprints/DataTable_Potions/STRUCT_Potion` _returnvalue_2))) _selected1)
            _
            (elif (`KismetStringLibrary.EqualEqual_StrStr` (`|GetEnumeratorNameAsString` (`.Ingredient2_30_192627634D47B4973D1B6FABB33C6976` (break `/Game/Blueprints/DataTable_Potions/STRUCT_Potion` _returnvalue_2))) _selected1)
              _
              (elif (not (`KismetStringLibrary.EqualEqual_StrStr` _selected1 (`|GetEnumeratorNameAsString` (`.Ingredient3_31_82459F4446A459161F6F9EB9688980DF` (break `/Game/Blueprints/DataTable_Potions/STRUCT_Potion` _returnvalue_2)))))
                (`KismetArrayLibrary.Array_RemoveItem` (`self.Possible Potions`) _array_element_2)))))))
    (`self.PotionArray`)
    (if (!= (`KismetArrayLibrary.Array_Length` (`self.Possible Potions`)) 0)
      (for _array_element_3 (`self.PossiblePotionsIntermidant`)
        (bind _returnvalue_3 (`|GetDataTableRow` "/Game/Blueprints/DataTable_Potions/DataTable_Potions_Truncated.DataTable_Potions_Truncated" _array_element_3)
          (:`then`
            (if (`KismetStringLibrary.EqualEqual_StrStr` (`|GetEnumeratorNameAsString` (`.Ingredient1_29_80935F3448C1E0AB5282968C8D72B828` (break `/Game/Blueprints/DataTable_Potions/STRUCT_Potion` _returnvalue_3))) _selected2)
              _
              (elif (`KismetStringLibrary.EqualEqual_StrStr` (`|GetEnumeratorNameAsString` (`.Ingredient2_30_192627634D47B4973D1B6FABB33C6976` (break `/Game/Blueprints/DataTable_Potions/STRUCT_Potion` _returnvalue_3))) _selected2)
                _
                (elif (not (`KismetStringLibrary.EqualEqual_StrStr` _selected2 (`|GetEnumeratorNameAsString` (`.Ingredient3_31_82459F4446A459161F6F9EB9688980DF` (break `/Game/Blueprints/DataTable_Potions/STRUCT_Potion` _returnvalue_3)))))
                  (`KismetArrayLibrary.Array_RemoveItem` (`self.Possible Potions`) _array_element_3)))))))
      (`self.PotionArray`)
      (if (!= (`KismetArrayLibrary.Array_Length` (`self.Possible Potions`)) 0)
        (for _array_element_4 (`self.PossiblePotionsIntermidant`)
          (bind _returnvalue_4 (`|GetDataTableRow` "/Game/Blueprints/DataTable_Potions/DataTable_Potions_Truncated.DataTable_Potions_Truncated" _array_element_4)
            (:`then`
              (if (`KismetStringLibrary.EqualEqual_StrStr` (`|GetEnumeratorNameAsString` (`.Ingredient1_29_80935F3448C1E0AB5282968C8D72B828` (break `/Game/Blueprints/DataTable_Potions/STRUCT_Potion` _returnvalue_4))) _selected3)
                _
                (elif (`KismetStringLibrary.EqualEqual_StrStr` (`|GetEnumeratorNameAsString` (`.Ingredient2_30_192627634D47B4973D1B6FABB33C6976` (break `/Game/Blueprints/DataTable_Potions/STRUCT_Potion` _returnvalue_4))) _selected3)
                  _
                  (elif (not (`KismetStringLibrary.EqualEqual_StrStr` _selected3 (`|GetEnumeratorNameAsString` (`.Ingredient3_31_82459F4446A459161F6F9EB9688980DF` (break `/Game/Blueprints/DataTable_Potions/STRUCT_Potion` _returnvalue_4)))))
                    (`KismetArrayLibrary.Array_RemoveItem` (`self.Possible Potions`) _array_element_4)))))))
        (if (!= (`KismetArrayLibrary.Array_Length` (`self.Possible Potions`)) 0)
          (return (`|GetArrayItem` (`self.Possible Potions`)))
          (else
            _)))))
  (return "Null"))

(fn `RunePotionCalculator`
  (returns (`Can Craft` :type "Array of Name"))
  (bind _selected2 (`self.Selected2`))
  (bind _selected3 (`self.Selected3`))
  (bind _selected1 (`self.Selected1`))
  (bind _possible_potions (`self.Possible Potions`))
  (`KismetArrayLibrary.Array_Clear` (`self.Possible Potions`))
  (bind _outrownames (`DataTableFunctionLibrary.GetDataTableRowNames` "/Game/Blueprints/DataTable_Potions/DataTable_Potions_Truncated.DataTable_Potions_Truncated"))
  (for _array_element _outrownames
    (bind _returnvalue (`|GetDataTableRow` "/Game/Blueprints/DataTable_Potions/DataTable_Potions_Truncated.DataTable_Potions_Truncated" _array_element)
      (:`then`
        (if (`KismetStringLibrary.EqualEqual_StrStr` (`|GetEnumeratorNameAsString` (`.Ingredient1_29_80935F3448C1E0AB5282968C8D72B828` (break `/Game/Blueprints/DataTable_Potions/STRUCT_Potion` _returnvalue))) _selected1)
          (`KismetArrayLibrary.Array_AddUnique` _possible_potions _array_element :!label _label)
          (elif (`KismetStringLibrary.EqualEqual_StrStr` (`|GetEnumeratorNameAsString` (`.Ingredient2_30_192627634D47B4973D1B6FABB33C6976` (break `/Game/Blueprints/DataTable_Potions/STRUCT_Potion` _returnvalue))) _selected1)
            (goto _label)
            (elif (`KismetStringLibrary.EqualEqual_StrStr` _selected1 (`|GetEnumeratorNameAsString` (`.Ingredient3_31_82459F4446A459161F6F9EB9688980DF` (break `/Game/Blueprints/DataTable_Potions/STRUCT_Potion` _returnvalue))))
              (goto _label)
              (else
                (`KismetArrayLibrary.Array_RemoveItem` _possible_potions _array_element))))))))
  (`self.PotionArray`)
  (if (!= (`KismetArrayLibrary.Array_Length` (`self.Possible Potions`)) 0)
    (for _array_element_2 (`self.PossiblePotionsIntermidant`)
      (bind _returnvalue_2 (`|GetDataTableRow` "/Game/Blueprints/DataTable_Potions/DataTable_Potions_Truncated.DataTable_Potions_Truncated" _array_element_2)
        (:`then`
          (if (`KismetStringLibrary.EqualEqual_StrStr` (`|GetEnumeratorNameAsString` (`.Ingredient1_29_80935F3448C1E0AB5282968C8D72B828` (break `/Game/Blueprints/DataTable_Potions/STRUCT_Potion` _returnvalue_2))) _selected2)
            _
            (elif (`KismetStringLibrary.EqualEqual_StrStr` (`|GetEnumeratorNameAsString` (`.Ingredient2_30_192627634D47B4973D1B6FABB33C6976` (break `/Game/Blueprints/DataTable_Potions/STRUCT_Potion` _returnvalue_2))) _selected2)
              _
              (elif (not (`KismetStringLibrary.EqualEqual_StrStr` _selected2 (`|GetEnumeratorNameAsString` (`.Ingredient3_31_82459F4446A459161F6F9EB9688980DF` (break `/Game/Blueprints/DataTable_Potions/STRUCT_Potion` _returnvalue_2)))))
                (`KismetArrayLibrary.Array_RemoveItem` (`self.Possible Potions`) _array_element_2)))))))
    (`self.PotionArray`)
    (if (!= (`KismetArrayLibrary.Array_Length` (`self.Possible Potions`)) 0)
      (for _array_element_3 (`self.PossiblePotionsIntermidant`)
        (bind _returnvalue_3 (`|GetDataTableRow` "/Game/Blueprints/DataTable_Potions/DataTable_Potions_Truncated.DataTable_Potions_Truncated" _array_element_3)
          (:`then`
            (if (`KismetStringLibrary.EqualEqual_StrStr` (`|GetEnumeratorNameAsString` (`.Ingredient1_29_80935F3448C1E0AB5282968C8D72B828` (break `/Game/Blueprints/DataTable_Potions/STRUCT_Potion` _returnvalue_3))) _selected3)
              _
              (elif (`KismetStringLibrary.EqualEqual_StrStr` (`|GetEnumeratorNameAsString` (`.Ingredient2_30_192627634D47B4973D1B6FABB33C6976` (break `/Game/Blueprints/DataTable_Potions/STRUCT_Potion` _returnvalue_3))) _selected3)
                _
                (elif (not (`KismetStringLibrary.EqualEqual_StrStr` _selected3 (`|GetEnumeratorNameAsString` (`.Ingredient3_31_82459F4446A459161F6F9EB9688980DF` (break `/Game/Blueprints/DataTable_Potions/STRUCT_Potion` _returnvalue_3)))))
                  (`KismetArrayLibrary.Array_RemoveItem` (`self.Possible Potions`) _array_element_3)))))))
      (if (!= (`KismetArrayLibrary.Array_Length` (`self.Possible Potions`)) 0)
        (return (`self.Possible Potions`))
        (else
          _))))
  (return))

(fn `Sigil Widget Closer`
  (`Widget.RemoveFromParent` (`self.Sigil_UI_Ref`)))

(fn `Sigil Widget Runner`
  (`UserWidget.AddToViewport` (`self.Sigil_UI_Ref`) 0))

(fn `UserConstructionScript`)

(fn `WidgetFunction`
  (bind _returnvalue (`|CreateWidget` "/Game/Blueprints/UI/UI_NPC_Text.UI_NPC_Text_C"))
  (bind _output_get (set `self.UI_NPC_TextRef` _returnvalue))
  (`UserWidget.AddToViewport` _output_get 0)
  (bind _returnvalue_2 (`|CreateWidget` "/Game/Blueprints/UI/UI_Sigil_Selector.UI_Sigil_Selector_C"))
  (set `self.Sigil_UI_Ref` _returnvalue_2)
  (bind _returnvalue_3 (`|CreateWidget` "/Game/Blueprints/UI/WB_MorterAndPestel.WB_MorterAndPestel_C"))
  (set `self.MortaAndPestle_UI_Ref` _returnvalue_3)
  (bind _returnvalue_4 (`|CreateWidget` "/Game/Blueprints/UI/UI_Sigil_Timer.UI_Sigil_Timer_C"))
  (set `self.SigilTimerWidgetRef` _returnvalue_4)
  (bind _returnvalue_5 (`|CreateWidget` "/Game/Stewart2/Inventory/Widgets/UMG_CraftingTableNew.UMG_CraftingTableNew_C" null null null))
  (set `self.CraftingWidgetRef` _returnvalue_5)
  (bind _returnvalue_6 (`|CreateWidget` "/Game/Blueprints/RuneWheel/UMG_RuneSelect.UMG_RuneSelect_C" null null))
  (set `self.RuneWidgetRef` _returnvalue_6))